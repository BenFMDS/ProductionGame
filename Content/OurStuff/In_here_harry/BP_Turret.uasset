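; BP_Turret is a turret actor whose Sphere component turns its barrel toward whatever the player's crosshair is on.
; Each Tick traces from the camera centre on the Visibility channel, ignoring the player pawn, and falls back to a distant point on a miss.
; The look-at is computed from that point back to the Sphere because the barrel faces -X, and RInterpTo smooths the turn by AimSpeed.
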(event `self.ReceiveTick`
  (params (DeltaSeconds :type "Float (single-precision)"))
  (bind _returnvalue (`GameplayStatics.GetPlayerCameraManager` 0))
  (bind _sphere (`self.Sphere`))
  (bind _returnvalue_2 (`PlayerCameraManager.GetCameraLocation` _returnvalue))
  (bind _returnvalue_3 (+ _returnvalue_2 (* (`KismetMathLibrary.GetForwardVector` (`PlayerCameraManager.GetCameraRotation` _returnvalue)) 100000.0)))
  ; Where is the crosshair? (screen centre = the camera's centre line)
  (if (`KismetSystemLibrary.IsValid` _returnvalue)
    ; Find what the crosshair is on (or a point far away if it's on the sky)
    (bind (_outhit _returnvalue_4) (`KismetSystemLibrary.LineTraceSingle` _returnvalue_2 _returnvalue_3 "TraceTypeQuery1" false (`|MakeArray` (`GameplayStatics.GetPlayerPawn` 0) :!type "Actor Object Reference")))
    (bind (_returnvalue_roll _returnvalue_pitch _returnvalue_yaw) (`KismetMathLibrary.BreakRotator` (`KismetMathLibrary.RInterpTo` (`SceneComponent.K2_GetComponentRotation` _sphere) (`KismetMathLibrary.FindLookAtRotation` (`KismetMathLibrary.SelectVector` (`.ImpactPoint` (`GameplayStatics.BreakHitResult` _outhit)) _returnvalue_3 _returnvalue_4) (`SceneComponent.K2_GetComponentLocation` _sphere)) DeltaSeconds (`self.AimSpeed`))))
    ; Turn the sphere so the barrel (its -X side) points there, smoothed by Aim Speed
    (`SceneComponent.K2_SetWorldRotation` _sphere (`KismetMathLibrary.MakeRotator` _returnvalue_roll _returnvalue_pitch _returnvalue_yaw) false false)))

(fn `UserConstructionScript`)