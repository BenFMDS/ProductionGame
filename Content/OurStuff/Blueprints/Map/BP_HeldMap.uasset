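; BP_HeldMap is a held map that the player raises while the map input is held and lowers on release.
; A timeline moves and tilts MapRoot, hiding it once fully lowered.
; A floor input pages the WBP_BlueprintMap shown in its widget component up or down.
; It also listens to PlayerQuestComponent conversation changes, collecting each conversation NPC uniquely into MetExhibits.
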(event `self.ReceiveBeginPlay`
  (bind _returnvalue (`GameplayStatics.GetPlayerController` 0))
  (bind _returnvalue_2 (`self.GetComponentByClass` (`GameplayStatics.GetPlayerController` 0) "/Script/ProductionGame.PlayerQuestComponent"))
  (bind _aswbp_blueprint_map (cast `/Game/OurStuff/Widgets/Map/WBP_BlueprintMap` (`WidgetComponent.GetUserWidgetObject` (`self.MapWidget`))))
  (set `self.Map` _aswbp_blueprint_map)
  (`SceneComponent.SetVisibility` (`self.MapRoot`) false true)
  (`self.EnableInput` _returnvalue)
  (`EnhancedInputSubsystemInterface.AddMappingContext` (pcsubsystem `EnhancedInputLocalPlayerSubsystem` _returnvalue) "/Game/Input/IMC_Map.IMC_Map" 1 (struct))
  (`/Engine/EditorBlueprintResources/StandardMacros.IsValid` _returnvalue_2
    (:`Is Valid`
      (bind _output_get (set `self.PlayerQuests` _returnvalue_2))
      (add `PlayerQuestComponent.OnConversationChanged` _output_get (`|CreateDelegate` :!event `OnConversationChanged`)))))

(event `EnhancedInput|/Game/Input/Actions/IA_Map`
  (params (ActionValue :type Boolean) (ElapsedSeconds :type "Float (double-precision)") (TriggeredSeconds :type "Float (double-precision)") (InputAction :type "InputAction Object Reference" :default "/Game/Input/Actions/IA_Map.IA_Map"))
  (:`Started`
    (`SceneComponent.SetVisibility` (`self.MapRoot`) true true)
    ; Raise/Lower Animations
    (bind (_direction _alpha) (`Timeline|Raise` :!label _label)
      (:`Update`
        (`SceneComponent.K2_SetRelativeLocationAndRotation` (`self.MapRoot`) (`KismetMathLibrary.VLerp` (`self.Lowered Loc`) (`self.RaisedLoc`) _alpha) (`KismetMathLibrary.MakeRotator` 0.0 (`KismetMathLibrary.Lerp` -25.0 -10.0 _alpha)) false false))
      (:`Finished`
        (if (`|EnumEquality` _direction "Backward")
          (`SceneComponent.SetVisibility` (`self.MapRoot`) false true)))))
  (:`Completed`
    (goto _label :!via `Reverse`)))

(event `EnhancedInput|/Game/Input/Actions/IA_MapFloor`
  (params (ActionValue :type "Float (double-precision)") (ElapsedSeconds :type "Float (double-precision)") (TriggeredSeconds :type "Float (double-precision)") (InputAction :type "InputAction Object Reference" :default "/Game/Input/Actions/IA_MapFloor.IA_MapFloor"))
  (bind _map (`self.Map`))
  (:`Triggered`
    (if (> ActionValue 0.0)
      (`/Game/OurStuff/Widgets/Map/WBP_BlueprintMap.NextFloor` _map)
      (else
        (`/Game/OurStuff/Widgets/Map/WBP_BlueprintMap.PrevFloor` _map)))))

(event `OnConversationChanged`
  (bind _npc (break `PlayerConversation` (`PlayerQuestComponent.Conversation` (`self.PlayerQuests`))))
  (`/Engine/EditorBlueprintResources/StandardMacros.IsValid` _npc
    (:`Is Valid`
      (`KismetArrayLibrary.Array_AddUnique` (`self.MetExhibits`) _npc))))

(fn `UserConstructionScript`)