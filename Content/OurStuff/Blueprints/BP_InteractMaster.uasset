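; BP_InteractMaster is a base-style interactable actor in what appears to be a robber game, with interaction text and a default Interact response that destroys it.
; The construction script caches the static mesh and uses InteractType to choose between a simulated physics body and a non-simulated WorldDynamic object.
; BeginPlay caches the BP_RobberGameState reference, and GetInteractData exposes InteractText to callers.
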(event `self.ReceiveBeginPlay`
  (bind _returnvalue (`GameplayStatics.GetActorOfClass` "/Game/OurStuff/Core/Player/Game/BP_RobberGameState.BP_RobberGameState_C"))
  (set `self.GameStateRef` _returnvalue))

(event `/Game/OurStuff/Core/InteractionSystem/BPI_Interaction.Interact`
  (params (InteractingPlayer :type "Actor Object Reference") (`ServerInteract?` :type Boolean))
  (`self.K2_DestroyActor`))

(fn `GetInteractData`
  (returns (InteractText :type String))
  (return (`self.Interact Text`)))

(fn `UserConstructionScript`
  (bind _mesh (`self.Mesh`))
  (bind _mesh_2 (`self.Mesh`))
  (set `self.SceneMesh` (`StaticMeshComponent.StaticMesh` (`self.Mesh`)))
  (if (`|EnumEquality` (`self.Interact Type`) "NewEnumerator1")
    (`PrimitiveComponent.SetSimulatePhysics` _mesh_2 true)
    (`PrimitiveComponent.SetCollisionObjectType` _mesh_2 "ECC_PhysicsBody")
    (else
      (`PrimitiveComponent.SetSimulatePhysics` _mesh false)
      (`PrimitiveComponent.SetCollisionObjectType` _mesh "ECC_WorldDynamic"))))