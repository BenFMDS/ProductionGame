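; BP_Guard is a networked guard character that holds a flashlight and reacts to alerts and hits.
; On BeginPlay it binds itself to its WBP_GuardMeter widget and attaches a spawned flashlight to a hand socket.
; Alerts and authority-side landed hits are forwarded to BP_GuardController for handling.
; The GuardState OnRep plays suspicious or chase sounds at the guard's location, and MC_PlayHit plays the hit montage.
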(event `self.ReceiveBeginPlay`
  (bind _aswbp_guard_meter (cast `/Game/OurStuff/Blueprints/Guard/WBP_GuardMeter` (`WidgetComponent.GetUserWidgetObject` (`self.MeterWidget`))))
  (set `/Game/OurStuff/Blueprints/Guard/WBP_GuardMeter.Guard` self _aswbp_guard_meter)
  (bind _returnvalue (`|SpawnActorFromClass` "/Game/OurStuff/Blueprints/Flashlight/BP_flashlight.BP_flashlight_C" (`SceneComponent.GetSocketTransform` (`self.Mesh`) "Hand_r_flashlight_socket" "RTS_World") "Undefined" "MultiplyWithRoot" null null))
  (`self.K2_AttachToComponent` _returnvalue (`self.Mesh`) "Hand_r_flashlight_socket" "SnapToTarget" "SnapToTarget" "SnapToTarget" true))

(event `OnHitLanded`
  (`/Engine/EditorBlueprintResources/ActorMacros.Switch Has Authority`
    (:`Authority`
      (bind _asbp_guard_controller (cast `/Game/OurStuff/Blueprints/Guard/BP_GuardController` (`self.GetController`)))
      (`/Game/OurStuff/Blueprints/Guard/BP_GuardController.HitLanded` _asbp_guard_controller))))

(event `MC_PlayHit`
  (`self.PlayAnimMontage` "/Game/OurStuff/Animations/AM_GuardHit.AM_GuardHit"))

(fn `OnRep_GuardState`
  (switch `/Game/OurStuff/Blueprints/Guard/E_GuardState` (`self.GuardState`)
    (:`NewEnumerator1`
      (`GameplayStatics.PlaySoundAtLocation` (`self.SuspiciousSound`) (`self.K2_GetActorLocation`) (struct) 1.0 1.0 0.0 null null null null))
    (:`NewEnumerator3`
      (`GameplayStatics.PlaySoundAtLocation` (`self.ChaseSound`) (`self.K2_GetActorLocation`) (struct) 1.0 1.0 0.0 null null null null))))

(fn `ReportAlert`
  (params (Location :type "Vector Structure") (AlertInstigator :type "Actor Object Reference"))
  (bind _asbp_guard_controller (cast `/Game/OurStuff/Blueprints/Guard/BP_GuardController` (`self.GetController`)))
  (`/Game/OurStuff/Blueprints/Guard/BP_GuardController.HandleAlert` _asbp_guard_controller Location AlertInstigator))

(fn `UserConstructionScript`)