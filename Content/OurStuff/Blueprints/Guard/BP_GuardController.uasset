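; AI controller for robber-hunting guards that runs BT_Guard and drives a Patrol, Suspicious, Investigate and Chase state machine.
; Each tick, sight fills a detection meter (scaled by player 0's crouch) or drains it, changing state and catching chased robbers within range.
; Hearing and game-state camera sightings, answered only by the nearest free guard, trigger investigation.
; State changes update the Blackboard, movement speed, focus and rotation mode.
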(event `self.ReceivePossess`
  (params (PossessedPawn :type "Pawn Object Reference"))
  (bind _asbp_guard (cast `/Game/OurStuff/Blueprints/Guard/BP_Guard` PossessedPawn))
  (set `self.Guard` _asbp_guard)
  (`self.RunBehaviorTree` "/Game/OurStuff/Blueprints/Guard/Behaviour/BT_Guard.BT_Guard")
  (bind _asbp_robber_game_state (cast `/Game/OurStuff/Core/Player/Game/BP_RobberGameState` (`GameplayStatics.GetGameState`)))
  (add `RobberGameState.OnInvestigate` _asbp_robber_game_state (`|CreateDelegate` :!event `OnCameraSighting`)))

(event `self.ReceiveTick`
  (params (DeltaSeconds :type "Float (single-precision)"))
  (`self.UpdateDetection` DeltaSeconds))

(event `self.AIPerception.OnTargetPerceptionUpdated`
  (params (Actor :type "Actor Object Reference") (Stimulus :type "AIStimulus Structure"))
  (bind (_age _expirationage _strength _stimuluslocation _receiverlocation _tag _bsuccessfullysensed) (break `AIStimulus` Stimulus))
  (bind _returnvalue (`AIPerceptionSystem.GetSenseClassForStimulus` Stimulus))
  (if (and (== _returnvalue "/Script/AIModule.AISense_Hearing") _bsuccessfullysensed)
    (`self.HandleAlert` _stimuluslocation Actor)))

(event `OnCameraSighting`
  (params (Location :type "Vector Structure") (ReportedBy :type "Actor Object Reference"))
  (bind _isnearest (`self.IsNearestFreeGuard` Location))
  (if _isnearest
    (`self.HandleAlert` Location ReportedBy)
    (`KismetSystemLibrary.PrintString` "Camera sighted player")))

(event `HitLanded`)

(fn `CatchRobber`
  (params (Robber :type "Actor Object Reference"))
  (bind _returnvalue (`self.GetComponentByClass` Robber "/Game/OurStuff/Blueprints/Guard/BPC_Caught.BPC_Caught_C"))
  (bind _guard (`self.Guard`))
  (`/Game/OurStuff/Blueprints/Guard/BP_Guard.MC_PlayHit` (`self.Guard`))
  (`/Engine/EditorBlueprintResources/StandardMacros.IsValid` _returnvalue
    (:`Is Valid`
      (`/Game/OurStuff/Blueprints/Guard/BPC_Caught.GetCaught` _returnvalue))
    (:`Is Not Valid`
      _))
  (`BlackboardComponent.ClearValue` (`AIBlueprintHelperLibrary.GetBlackboard` null) "TargetActor")
  (set `/Game/OurStuff/Blueprints/Guard/BP_Guard.TargetRobber` null _guard)
  (set `/Game/OurStuff/Blueprints/Guard/BP_Guard.Detection` 0.0 _guard)
  (set `self.TimeSinceSeen` 0.0)
  (`BlackboardComponent.SetValueAsVector` (`AIBlueprintHelperLibrary.GetBlackboard` null) "LastKnownLocation" (`self.K2_GetActorLocation` _guard))
  (`self.SetGuardState` "NewEnumerator2"))

(fn `FindSeenRobber`
  (returns (Robber :type "Character Object Reference"))
  (locals (Best :type "Character Object Reference") (BestDistance :type "Float (double-precision)" :default 9999999.0))
  (set `self.SeenActors` (`AIPerceptionComponent.GetCurrentlyPerceivedActors` (`self.AIPerception`) "/Script/AIModule.AISense_Sight"))
  (bind _ascharacter (cast `Character` (`BlackboardComponent.GetValueAsObject` (`AIBlueprintHelperLibrary.GetBlackboard` null) "TargetActor"))
    (:`then`
      (if (`KismetArrayLibrary.Array_Contains` (`self.SeenActors`) _ascharacter)
        (return _ascharacter)
        (else
          _)))
    (:`CastFailed`
      _))
  (for _array_element (`self.SeenActors`)
    (bind _ascharacter_2 (cast `Character` _array_element))
    (if (`Pawn.IsPlayerControlled` _ascharacter_2)
      (if (not (`self.IsRobberCaught` _ascharacter_2))
        (bind _returnvalue (`self.GetDistanceTo` _ascharacter_2 (`self.Guard`)))
        (if (< _returnvalue (`local.BestDistance`))
          (bind _output_get (set `local.Best` _ascharacter_2))
          (set `local.BestDistance` _returnvalue)
          (return _output_get))))))

(fn `HandleAlert`
  (params (Location :type "Vector Structure") (AlertInstigator :type "Actor Object Reference"))
  (switch `/Game/OurStuff/Blueprints/Guard/E_GuardState` (`/Game/OurStuff/Blueprints/Guard/BP_Guard.GuardState` (`self.Guard`))
    (:`NewEnumerator0`
      _)
    (:`NewEnumerator2`
      _))
  (`BlackboardComponent.SetValueAsVector` (`AIBlueprintHelperLibrary.GetBlackboard` null) "LastKnownLocation" Location)
  (bind _ascharacter (cast `Character` AlertInstigator)
    (:`then`
      (if (`Pawn.IsPlayerControlled` _ascharacter)
        (set `/Game/OurStuff/Blueprints/Guard/BP_Guard.TargetRobber` _ascharacter (`self.Guard`))
        (else
          (set `/Game/OurStuff/Blueprints/Guard/BP_Guard.TargetRobber` null (`self.Guard`) :!label _label))))
    (:`CastFailed`
      (goto _label)))
  (`self.SetGuardState` "NewEnumerator2"))

(fn `IsNearestFreeGuard`
  (params (Location :type "Vector Structure"))
  (returns (IsNearest :type Boolean))
  (locals (BestGuard :type "/Game/OurStuff/Blueprints/Guard/BP_Guard Object Reference") (BestDistance :type "Float (double-precision)"))
  (set `local.BestDistance` 1000000.0)
  (set `local.BestGuard` null)
  (bind _outactors (`GameplayStatics.GetAllActorsOfClass` "/Game/OurStuff/Blueprints/Guard/BP_Guard.BP_Guard_C"))
  (for _array_element _outactors
    (bind _guardstate (`/Game/OurStuff/Blueprints/Guard/BP_Guard.GuardState` _array_element))
    (if (or (`|EnumEquality` _guardstate "NewEnumerator0") (`|EnumEquality` _guardstate "NewEnumerator2"))
      (bind _returnvalue (`KismetMathLibrary.Vector_Distance` (`self.K2_GetActorLocation` _array_element) Location))
      (if (< _returnvalue (`local.BestDistance`))
        (set `local.BestDistance` _returnvalue)
        (set `local.BestGuard` _array_element))))
  (return (== (`local.BestGuard`) (`self.Guard`))))

(fn `IsRobberCaught`
  (params (Robber :type "Actor Object Reference"))
  (returns (Caught :type Boolean))
  (bind _returnvalue (`self.GetComponentByClass` Robber "/Game/OurStuff/Blueprints/Guard/BPC_Caught.BPC_Caught_C"))
  (`/Engine/EditorBlueprintResources/StandardMacros.IsValid` _returnvalue
    (:`Is Valid`
      (return (`/Game/OurStuff/Blueprints/Guard/BPC_Caught.IsCaught` _returnvalue)))
    (:`Is Not Valid`
      (return false))))

(fn `SetGuardState`
  (params (NewState :type "/Game/OurStuff/Blueprints/Guard/E_GuardState Enum" :default "NewEnumerator0"))
  (locals (KeyName :type Name :default "GuardState"))
  (bind _guard (`self.Guard`))
  (bind _guard_2 (`self.Guard`))
  (bind _guard_3 (`self.Guard`))
  (bind _guard_4 (`self.Guard`))
  (if (`|EnumInequality` NewState (`/Game/OurStuff/Blueprints/Guard/BP_Guard.GuardState` _guard_4))
    (`BlackboardComponent.SetValueAsEnum` (`AIBlueprintHelperLibrary.GetBlackboard` null) (`local.KeyName`) NewState)
    (bind _output_get (set `/Game/OurStuff/Blueprints/Guard/BP_Guard.GuardState` NewState _guard_4))
    (switch `/Game/OurStuff/Blueprints/Guard/E_GuardState` _output_get
      (:`NewEnumerator0`
        (set `/Game/OurStuff/Blueprints/Guard/BP_Guard.TargetRobber` null _guard)
        (set `CharacterMovementComponent.MaxWalkSpeed` (`/Game/OurStuff/Blueprints/Guard/BP_Guard.WalkSpeed` _guard) (`Character.CharacterMovement` _guard))
        (`self.K2_ClearFocus`)
        (`self.SetRotationMode` false))
      (:`NewEnumerator1`
        (`self.StopMovement`)
        (bind _asactor (cast `Actor` (`BlackboardComponent.GetValueAsObject` (`AIBlueprintHelperLibrary.GetBlackboard` null) "TargetActor")))
        (`self.K2_SetFocus` _asactor)
        (`self.SetRotationMode` true))
      (:`NewEnumerator2`
        (set `CharacterMovementComponent.MaxWalkSpeed` (`/Game/OurStuff/Blueprints/Guard/BP_Guard.InvestigateSpeed` _guard_2) (`Character.CharacterMovement` _guard_2))
        (`self.K2_ClearFocus`)
        (`self.SetRotationMode` false))
      (:`NewEnumerator3`
        (set `CharacterMovementComponent.MaxWalkSpeed` (`/Game/OurStuff/Blueprints/Guard/BP_Guard.RunSpeed` _guard_3) (`Character.CharacterMovement` _guard_3))
        (`self.K2_ClearFocus`)
        (`self.SetRotationMode` false)))))

(fn `SetRotationMode`
  (params (FaceTarget :type Boolean))
  (bind _charactermovement (`Character.CharacterMovement` (`self.Guard`)))
  (set `CharacterMovementComponent.bOrientRotationToMovement` (not FaceTarget) _charactermovement)
  (set `CharacterMovementComponent.bUseControllerDesiredRotation` FaceTarget _charactermovement))

(fn `UpdateDetection`
  (params (DeltaSeconds :type "Float (double-precision)"))
  (locals (Seen :type "Character Object Reference") (Rate :type "Float (double-precision)") (Target :type "Actor Object Reference"))
  (bind _seen (`local.Seen`))
  (bind _guard (`self.Guard`))
  (bind _guard_2 (`self.Guard`))
  (bind _guard_3 (`self.Guard`))
  (bind _guard_4 (`self.Guard`))
  (bind _guard_5 (`self.Guard`))
  (bind _guardstate (`/Game/OurStuff/Blueprints/Guard/BP_Guard.GuardState` (`self.Guard`)))
  (bind _guardstate_2 (`/Game/OurStuff/Blueprints/Guard/BP_Guard.GuardState` _guard_2))
  (`/Engine/EditorBlueprintResources/StandardMacros.IsValid` (`self.Guard`)
    (:`Is Valid`
      (bind _asactor (cast `Actor` (`BlackboardComponent.GetValueAsObject` (`AIBlueprintHelperLibrary.GetBlackboard` null) "TargetActor"))
        (:`then`
          (set `local.Target` _asactor))
        (:`CastFailed`
          _))
      (if (and (`|EnumEquality` (`/Game/OurStuff/Blueprints/Guard/BP_Guard.GuardState` _guard_4) "NewEnumerator3") (`KismetSystemLibrary.IsValid` (`local.Target`)) (<= (`self.GetDistanceTo` _guard_4 (`local.Target`)) (`self.CatchRadius`)))
        (`self.CatchRobber` (`local.Target`))
        (return)
        (else
          (bind _robber (`self.FindSeenRobber`))
          (bind _output_get (set `local.Seen` _robber))
          (if (`KismetSystemLibrary.IsValid` _output_get)
            ; True Branch: Someone is Seen
            (`BlackboardComponent.SetValueAsObject` (`AIBlueprintHelperLibrary.GetBlackboard` null) "TargetActor" _seen)
            (set `/Game/OurStuff/Blueprints/Guard/BP_Guard.TargetRobber` _seen (`self.Guard`))
            (`BlackboardComponent.SetValueAsVector` (`AIBlueprintHelperLibrary.GetBlackboard` null) "LastKnownLocation" (`self.K2_GetActorLocation` (`local.Seen`)))
            (set `self.TimeSinceSeen` 0.0)
            ;; Fill Rate: Crouch Multiplier Reduces the Detection Rate
            (set `local.Rate` (* (`self.DetectionRateUp`) (`KismetMathLibrary.SelectFloat` (`self.CrouchMultiplier`) 1.0 (`Character.bIsCrouched` (`GameplayStatics.GetPlayerCharacter` 0)))))
            (set `/Game/OurStuff/Blueprints/Guard/BP_Guard.Detection` (`KismetMathLibrary.FClamp` (+ (`/Game/OurStuff/Blueprints/Guard/BP_Guard.Detection` _guard_5) (* (`local.Rate`) DeltaSeconds)) 0.0 (`/Game/OurStuff/Blueprints/Guard/BP_Guard.DetectionMax` _guard_5)) (`self.Guard`))
            ;; Set Guard States
            (if (>= (`/Game/OurStuff/Blueprints/Guard/BP_Guard.Detection` _guard_3) (`/Game/OurStuff/Blueprints/Guard/BP_Guard.DetectionMax` _guard_3))
              (`self.SetGuardState` "NewEnumerator3")
              (elif (or (`|EnumEquality` _guardstate "NewEnumerator0") (`|EnumEquality` _guardstate "NewEnumerator2"))
                (`self.SetGuardState` "NewEnumerator1")))
            (else
              ; False Branch: Nobody is Seen
              (set `self.TimeSinceSeen` (+ (`self.TimeSinceSeen`) DeltaSeconds))
              (set `/Game/OurStuff/Blueprints/Guard/BP_Guard.Detection` (`KismetMathLibrary.FClamp` (- (`/Game/OurStuff/Blueprints/Guard/BP_Guard.Detection` _guard) (* (`self.DetectionRateDown`) DeltaSeconds)) 0.0 (`/Game/OurStuff/Blueprints/Guard/BP_Guard.DetectionMax` _guard)) _guard_2)
              (if (and (or (`|EnumEquality` _guardstate_2 "NewEnumerator1") (`|EnumEquality` _guardstate_2 "NewEnumerator3")) (>= (`self.TimeSinceSeen`) (`self.LoseSightTime`)))
                (`self.SetGuardState` "NewEnumerator2")))))))
    (:`Is Not Valid`
      (return))))

(fn `UserConstructionScript`)