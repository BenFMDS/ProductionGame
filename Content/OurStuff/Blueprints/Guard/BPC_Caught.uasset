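; BPC_Caught is a character component that handles a robber getting caught, knocking them out and sending them to jail.
; GetCaught stops any physics carry, ragdolls the mesh with input disabled, fades the camera out and starts a knockout timer.
; The timer teleports the character to a random BP_JailPoint, restores the mesh transform and collision cached at BeginPlay, re-enables input and fades back in.
; MC and Client event prefixes separate shared body changes from local camera effects.
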(event `self.ReceiveBeginPlay`
  (bind _ascharacter (cast `Character` (`self.GetOwner`)))
  (bind _output_get (set `self.OwnerChar` _ascharacter))
  (bind _mesh (`Character.Mesh` _output_get))
  (set `self.MeshRelLocation` (`SceneComponent.RelativeLocation` _mesh))
  (set `self.MeshRelRotation` (`SceneComponent.RelativeRotation` _mesh))
  (set `self.MeshProfile` (`PrimitiveComponent.GetCollisionProfileName` _mesh)))

(event `GetCaught`
  (bind _returnvalue (`Actor.GetComponentByClass` (`self.GetOwner`) "/Game/OurStuff/Core/InteractionSystem/BPC_PhysicsCarry.BPC_PhysicsCarry_C"))
  (if (not (`self.IsCaught`))
    (set `self.IsCaught` true)
    (`/Engine/EditorBlueprintResources/StandardMacros.IsValid` _returnvalue
      (:`Is Valid`
        (`/Game/OurStuff/Core/InteractionSystem/BPC_PhysicsCarry.StopCarry` _returnvalue))
      (:`Is Not Valid`
        _))
    (`self.MC_Ragdoll`)
    (`self.Client_FadeOut`)
    (`KismetSystemLibrary.K2_SetTimerDelegate` (delegate `FinishCaught`) (`self.KnockoutTime`))))

(event `FinishCaught`
  (bind _ownerchar (`self.OwnerChar`))
  (bind _returnvalue (`Actor.GetComponentByClass` _ownerchar "/Game/OurStuff/Core/InteractionSystem/BPC_PhysicsCarry.BPC_PhysicsCarry_C"))
  (`/Engine/EditorBlueprintResources/StandardMacros.IsValid` _returnvalue
    (:`Is Valid`
      (`/Game/OurStuff/Core/InteractionSystem/BPC_PhysicsCarry.StopCarry` _returnvalue))
    (:`Is Not Valid`
      _))
  (bind _outactors (`GameplayStatics.GetAllActorsOfClass` "/Game/OurStuff/Blueprints/Guard/BP_JailPoint.BP_JailPoint_C"))
  (if (> (`KismetArrayLibrary.Array_Length` _outactors) 0)
    (bind _outitem (`KismetArrayLibrary.Array_Random` _outactors))
    (bind _returnvalue_2 (`Actor.K2_GetActorRotation` _outitem))
    (set `self.JailRot` _returnvalue_2)
    (`Actor.K2_TeleportTo` _ownerchar (`Actor.K2_GetActorLocation` _outitem) _returnvalue_2)
    (`self.MC_Recover`)
    (`self.Client_FadeIn` (`self.JailRot`))
    (set `self.IsCaught` false)))

(event `MC_Ragdoll`
  (bind _ownerchar (`self.OwnerChar`))
  (bind _ownerchar_2 (`self.OwnerChar`))
  (bind _mesh (`Character.Mesh` _ownerchar))
  ; Ragdoll
  (`MovementComponent.StopMovementImmediately` (`Character.CharacterMovement` _ownerchar))
  (`PrimitiveComponent.SetCollisionProfileName` _mesh "Ragdoll" true)
  (`PrimitiveComponent.SetSimulatePhysics` _mesh true)
  (if (`Pawn.IsLocallyControlled` _ownerchar)
    (bind _asrobber_controller (cast `RobberController` (`Pawn.GetController` _ownerchar_2)))
    (`Actor.DisableInput` _ownerchar_2 _asrobber_controller)))

(event `Client_FadeOut`
  ; Camera Fades
  (`KismetSystemLibrary.Delay` 1.0)
  (bind _asrobber_controller (cast `RobberController` (`Pawn.GetController` (`self.OwnerChar`))))
  (`PlayerCameraManager.StartCameraFade` :`self` (`PlayerController.PlayerCameraManager` _asrobber_controller) :`ToAlpha` 1.0 :`Duration` 1.0 :`bHoldWhenFinished` true))

(event `Client_FadeIn`
  (params (Rot :type "Rotator Structure"))
  (bind _returnvalue (`Pawn.GetController` (`self.OwnerChar`)))
  ; Camera Fades
  (`Controller.SetControlRotation` _returnvalue Rot)
  (bind _asrobber_controller (cast `RobberController` _returnvalue))
  (`PlayerCameraManager.StartCameraFade` :`self` (`PlayerController.PlayerCameraManager` _asrobber_controller) :`FromAlpha` 1.0 :`Duration` 1.0))

(event `MC_Recover`
  (bind _ownerchar (`self.OwnerChar`))
  (bind _ownerchar_2 (`self.OwnerChar`))
  (bind _ownerchar_3 (`self.OwnerChar`))
  (bind _mesh (`Character.Mesh` _ownerchar))
  ; After Capture
  (`PrimitiveComponent.SetSimulatePhysics` _mesh false)
  (`SceneComponent.K2_AttachToComponent` _mesh (`Character.CapsuleComponent` _ownerchar) "None" "KeepRelative" "KeepRelative" "KeepRelative" false)
  (`SceneComponent.K2_SetRelativeLocationAndRotation` _mesh (`self.MeshRelLocation`) (`self.MeshRelRotation`) false false)
  (`PrimitiveComponent.SetCollisionProfileName` _mesh (`self.MeshProfile`) true)
  (`CharacterMovementComponent.SetMovementMode` (`Character.CharacterMovement` _ownerchar_2) "MOVE_Walking" 0)
  (if (`Pawn.IsLocallyControlled` _ownerchar_2)
    (bind _asrobber_controller (cast `RobberController` (`Pawn.GetController` _ownerchar_3)))
    (`Actor.EnableInput` _ownerchar_3 _asrobber_controller)))