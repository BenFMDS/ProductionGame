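; Controller for a wire-cutting puzzle in which wires must be cut in the order of the Wires array.
; OnWireCut compares the selected wire's Index to the current step, advancing on a match or resetting every wire through RPReset on a mistake.
; After the last step it sets IsComplete and notifies PuzzleObj through BPI_PuzzleSolver.
; IsComplete has an empty RepNotify, and feedback is print strings only.
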(fn `On Wire Cut`
  (bind _puzzleobj (`self.PuzzleObj`))
  (bind _wirestep (`self.WireStep`))
  (bind _wires (`self.Wires`))
  (if (`self.Is Complete`)
    (`KismetSystemLibrary.PrintString` "Puzzle Completed Already")
    (else
      (`/Engine/EditorBlueprintResources/StandardMacros.CompareInt` (`/Game/OurStuff/Blueprints/Puzzles/Wires/BP_Wire.Index` (`self.SelectedWire`)) (`/Game/OurStuff/Blueprints/Puzzles/Wires/BP_Wire.Index` (`|GetArrayItem` _wires _wirestep))
        (:`>`
          (`KismetSystemLibrary.PrintString` "Puzzle Failed" :!label _label)
          (`self.ResetWire`))
        (:`==`
          (set `self.WireStep` (+ _wirestep 1))
          (`/Engine/EditorBlueprintResources/StandardMacros.CompareInt` _wirestep (`KismetArrayLibrary.Array_Length` _wires)
            (:`>`
              _)
            (:`==`
              _))
          (set `self.Is Complete` true)
          (`KismetSystemLibrary.PrintString` "Puzzle Complete")
          (if (`KismetSystemLibrary.DoesImplementInterface` _puzzleobj "/Game/OurStuff/Blueprints/Puzzles/BPI_PuzzleSolver.BPI_PuzzleSolver_C")
            (message `/Game/OurStuff/Blueprints/Puzzles/BPI_PuzzleSolver.PuzzleSolved` _puzzleobj)))
        (:`<`
          (goto _label))))))

(fn `OnRep_Is Complete`)

(fn `ResetWire`
  (set `self.WireStep` 0)
  (set `self.SelectedWire` null)
  (for _array_element (`self.Wires`)
    (`/Game/OurStuff/Blueprints/Puzzles/Wires/BP_Wire.RP_Reset` _array_element))
  (`KismetSystemLibrary.PrintString` "Puzzle Reset"))

(fn `UserConstructionScript`)