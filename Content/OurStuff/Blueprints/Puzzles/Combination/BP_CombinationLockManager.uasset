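; BP_CombinationLockManager runs a four-digit combination lock puzzle that players solve by pressing buttons.
; On authority, each press increments the digit matching that button's index, wrapping after nine, then checks Input against Correct.
; A match marks the lock complete, blocking further presses, and calls Solve on Puzzle to open its targets, such as doors, chests or quests.
; Input's RepNotify refreshes the four text displays on clients.
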(event `self.ReceiveBeginPlay`
  (`self.UpdateVis`))

(event `ButtonPressed`
  (params (Button :type "/Game/OurStuff/Blueprints/Puzzles/Combination/BP_CombinationButton Object Reference"))
  (bind _input (`self.Input`))
  (bind _returnvalue (`KismetArrayLibrary.Array_Find` (`self.Buttons`) Button))
  (bind _output (`|GetArrayItem` _input _returnvalue))
  (`/Engine/EditorBlueprintResources/ActorMacros.Switch Has Authority`
    (:`Authority`
      (if (`self.Is Complete`)
        _
        (elif (!= _returnvalue -1)
          (if (>= _output 9)
            (`KismetArrayLibrary.Array_Set` _input _returnvalue)
            (`self.UpdateVis`)
            (`self.CheckPuzzle`)
            (else
              (bind _result (`/Engine/EditorBlueprintResources/StandardMacros.IncrementInt` _output)
                (:`  `
                  (`KismetArrayLibrary.Array_Set` _input _returnvalue _result)
                  (`self.UpdateVis`)
                  (`self.CheckPuzzle`))))))))))

(event `CheckPuzzle`
  (if (`KismetArrayLibrary.Array_Identical` (`self.Correct`) (`self.Input`))
    (set `self.Is Complete` true)
    (`KismetSystemLibrary.PrintString` "Puzzle Complete")
    ;[1 0.85 0.3] PUZZLE QUESTS: was Door -> OpenDoor. Now Puzzle -> Solve, so this puzzle can open anything in its Solve Targets (doors, chests, quests). Targets need BPI_PuzzleSolver.
    (`RobberPuzzleComponent.Solve` (`self.Puzzle`) null)))

(event `UpdateVis`
  (bind _input (`self.Input`))
  (`TextRenderComponent.K2_SetText` (`self.1`) (`|GenericToText` (`|GetArrayItem` _input)))
  (`TextRenderComponent.K2_SetText` (`self.2`) (`|GenericToText` (`|GetArrayItem` _input 1)))
  (`TextRenderComponent.K2_SetText` (`self.3`) (`|GenericToText` (`|GetArrayItem` _input 2)))
  (`TextRenderComponent.K2_SetText` (`self.4`) (`|GenericToText` (`|GetArrayItem` _input 3))))

(fn `Check Puzzle Complete`)

(fn `OnRep_Correct`)

(fn `OnRep_Input`
  (`self.UpdateVis`))

(fn `OnRep_Is Complete`)

(fn `UserConstructionScript`)