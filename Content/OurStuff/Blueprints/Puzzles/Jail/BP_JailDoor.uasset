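; Jail puzzle door that slides open when interacted with and closes itself after a set open time.
; Interact runs only with authority, setting the DoorOpen RepNotify variable and starting a timer that clears it.
; OnRep_DoorOpen plays or reverses the DoorMove timeline, which lerps the actor from its BeginPlay location toward that location plus OpenOffset.
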(event `self.ReceiveBeginPlay`
  (`parent.ReceiveBeginPlay`)
  (set `self.ClosedLocation` (`self.K2_GetActorLocation`)))

(event `AnimateDoor`
  (if (`self.DoorOpen`)
    (bind (_direction _alpha) (`Timeline|DoorMove` :!label _label)
      (:`Update`
        (`self.K2_SetActorLocation` (`KismetMathLibrary.VLerp` (`self.ClosedLocation`) (+ (`self.ClosedLocation`) (`self.OpenOffset`)) _alpha))))
    (else
      (goto _label :!via `Reverse`))))

(event `OpenDoor`
  (if (not (`self.DoorOpen`))
    (set `self.DoorOpen` true)
    (`KismetSystemLibrary.K2_SetTimerDelegate` (delegate `CloseDoor`) (`self.OpenTime`))))

(event `CloseDoor`
  (set `self.DoorOpen` false))

(event `/Game/OurStuff/Core/InteractionSystem/BPI_Interaction.Interact`
  (params (InteractingPlayer :type "Actor Object Reference") (`ServerInteract?` :type Boolean))
  (`/Engine/EditorBlueprintResources/ActorMacros.Switch Has Authority`
    (:`Authority`
      (`self.OpenDoor`))))

(fn `OnRep_DoorOpen`
  (`self.AnimateDoor`))

(fn `UserConstructionScript`
  (`parent.UserConstructionScript`))