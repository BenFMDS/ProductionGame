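; BP_LockPicker is a held robber tool for picking code locks.
; On Use, the locally controlled holder traces from the camera to cache any BP_KeyPadDoor, then always fires the server event RP_LickPickToggle.
; The server calls StartLockPick, which per the notes finds the nearest code lock itself, then after a stationary delay opens it, plays noise and adds heat.
; The old IsPicking and Door validity branch remains unplugged.
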(event `self.Use`
  (params (HitLocation :type "Vector Structure") (HitActor :type "Actor Object Reference") (`Impact Point` :type "Vector Structure"))
  ;[1 0.85 0.3] PUZZLE QUESTS: the server event went Branch -> Is Valid(Door) -> nothing. It calls StartLockPick now: the nearest code lock in front of whoever holds this, 5 s (stay put), then it opens, plays the noise maker's sound there and adds heat. The old Branch/IsPicking nodes are unplugged, not deleted.
  (bind _asbp_robber_character (cast `/Game/OurStuff/Core/Player/Game/BP_RobberCharacter` (`self.HeldBy`)))
  (if (`Pawn.IsLocallyControlled` _asbp_robber_character)
    (bind _outlocation (`self.GetActorEyesViewPoint` _asbp_robber_character))
    (bind _outhit (`KismetSystemLibrary.LineTraceSingle` _outlocation (+ _outlocation (* (`SceneComponent.GetForwardVector` (`ProductionGameCharacter.FirstPersonCameraComponent` _asbp_robber_character)) (`self.Dist`))) "TraceTypeQuery1"))
    (bind _asbp_key_pad_door (cast `/Game/OurStuff/Blueprints/Props/KeyPad/BP_KeyPadDoor` (`.HitActor` (`GameplayStatics.BreakHitResult` _outhit)))
      (:`then`
        ;[1 0.85 0.3] PUZZLE QUESTS: the client found the door and never told the server. Now Use always sends RP_LickPickToggle; the server finds the code lock itself, so this works on BP_CodeLock (Door here only knows BP_KeyPadDoor).
        (set `self.Door` _asbp_key_pad_door))
      (:`CastFailed`
        (set `self.Door` null)))
    (`self.RP_LickPickToggle`)))

(event `RP_LickPickToggle`
  ;[1 0.85 0.3] PUZZLE QUESTS: the server event went Branch -> Is Valid(Door) -> nothing. It calls StartLockPick now: the nearest code lock in front of whoever holds this, 5 s (stay put), then it opens, plays the noise maker's sound there and adds heat. The old Branch/IsPicking nodes are unplugged, not deleted.
  (`RobberPuzzleComponent.StartLockPick` self))

(fn `UserConstructionScript`
  (`parent.UserConstructionScript`))