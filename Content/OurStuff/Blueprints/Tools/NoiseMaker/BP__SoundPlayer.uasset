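; Noise maker tool that lets a robber holding it play a sound at an aimed world location.
; While held, Tick line-traces from the local robber's view to set the target and move the indicator, hiding it on a hit.
; Use passes the target to RP_NoiseMaker, which checks cooldown and range, then calls RPM_PlaySound.
; The range check and playback read the TargetLocation variable, leaving the passed Location unused.
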(event `RP_UpdateIndicator`
  (bind _sound_indicator (`self.Sound Indicator`))
  (bind _asbp_robber_character (cast `/Game/OurStuff/Core/Player/Game/BP_RobberCharacter` (`self.HeldBy`)))
  (if (`Pawn.IsLocallyControlled` _asbp_robber_character)
    (bind (_outlocation _outrotation) (`self.GetActorEyesViewPoint` _asbp_robber_character))
    (bind (_outhit _returnvalue) (`KismetSystemLibrary.LineTraceSingle` _outlocation (+ _outlocation (* (`SceneComponent.GetForwardVector` (`ProductionGameCharacter.FirstPersonCameraComponent` _asbp_robber_character)) (`self.Dist`))) "TraceTypeQuery1"))
    (if _returnvalue
      (bind _output_get (set `self.Target Location` (`.ImpactPoint` (`GameplayStatics.BreakHitResult` _outhit))))
      (set `self.ValidTarget` true)
      (`SceneComponent.K2_SetWorldLocationAndRotation` _sound_indicator _output_get _outrotation false false)
      (`SceneComponent.SetHiddenInGame` _sound_indicator true false)
      (else
        (`SceneComponent.SetHiddenInGame` (`self.Sound Indicator`) false false)))))

(event `self.ReceiveTick`
  (params (DeltaSeconds :type "Float (single-precision)"))
  (bind _heldby (`self.HeldBy`))
  (`/Engine/EditorBlueprintResources/StandardMacros.IsValid` _heldby
    (:`Is Valid`
      (bind _asbp_robber_character (cast `/Game/OurStuff/Core/Player/Game/BP_RobberCharacter` _heldby))
      (if (`Pawn.IsLocallyControlled` _asbp_robber_character)
        (`self.RP_UpdateIndicator`)))
    (:`Is Not Valid`
      (`SceneComponent.SetHiddenInGame` (`self.Sound Indicator`) false false))))

(event `self.Use`
  (params (HitLocation :type "Vector Structure") (HitActor :type "Actor Object Reference") (`Impact Point` :type "Vector Structure"))
  (bind _heldby (`self.HeldBy`))
  (`/Engine/EditorBlueprintResources/StandardMacros.IsValid` _heldby
    (:`Is Valid`
      (bind _asbp_robber_character (cast `/Game/OurStuff/Core/Player/Game/BP_RobberCharacter` _heldby))
      (if (`Controller.IsLocalController` (`Pawn.GetController` _asbp_robber_character))
        (`self.RP_NoiseMaker` (`self.Target Location`))))))

(event `RP_NoiseMaker`
  (params (Location :type "Vector Structure"))
  (bind _returnvalue (`KismetSystemLibrary.GetGameTimeInSeconds`))
  (bind _heldby (`self.HeldBy`))
  (`/Engine/EditorBlueprintResources/StandardMacros.IsValid` _heldby
    (:`Is Valid`
      (bind _asbp_robber_character (cast `/Game/OurStuff/Core/Player/Game/BP_RobberCharacter` _heldby))
      (if (>= _returnvalue (`self.NextTime`))
        (if (>= (`self.Dist`) (`KismetMathLibrary.Vector_Distance` (`self.Target Location`) (`SceneComponent.K2_GetComponentLocation` (`Character.CapsuleComponent` _asbp_robber_character))))
          (set `self.NextTime` (+ (`self.CoolDown`) _returnvalue))
          (`self.RPM_PlaySound`))))))

(event `RPM_PlaySound`
  (`GameplayStatics.PlaySoundAtLocation` (`self.Sound`) (`self.Target Location`) (struct) 1.0 1.0 0.0 null null null null))

(fn `UserConstructionScript`
  (`parent.UserConstructionScript`))