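; BP_Holdable is an item actor that robber characters can pick up and hold.
; Interact calls Pickup on the interacting robber, gated on HeldBy being valid.
; The HeldBy RepNotify runs ApplyHeldState, which either disables physics and collision and attaches to the holder's HoldPoint with HoldOffset, or detaches and restores both.
; Use only prints the name of the actor it hits.
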(event `self.ReceiveBeginPlay`
  (`parent.ReceiveBeginPlay`))

(event `/Game/OurStuff/Core/InteractionSystem/BPI_Interaction.Interact`
  (params (InteractingPlayer :type "Actor Object Reference") (`ServerInteract?` :type Boolean))
  (if `ServerInteract?`
    _
    (else
      _))
  (if (`KismetSystemLibrary.IsValid` (`self.HeldBy`))
    (bind _asbp_robber_character (cast `/Game/OurStuff/Core/Player/Game/BP_RobberCharacter` InteractingPlayer))
    (`/Game/OurStuff/Core/Player/Game/BP_RobberCharacter.Pickup` _asbp_robber_character self)))

(fn `ApplyHeldState`
  (bind _mesh (`self.Mesh`))
  (bind _mesh_2 (`self.Mesh`))
  (`/Engine/EditorBlueprintResources/StandardMacros.IsValid` (`self.HeldBy`)
    (:`Is Valid`
      (`PrimitiveComponent.SetSimulatePhysics` _mesh_2 false)
      (`PrimitiveComponent.SetCollisionEnabled` _mesh_2 "NoCollision")
      (bind _asbp_robber_character (cast `/Game/OurStuff/Core/Player/Game/BP_RobberCharacter` (`self.HeldBy`)))
      (`self.K2_AttachToComponent` (`/Game/OurStuff/Core/Player/Game/BP_RobberCharacter.HoldPoint` _asbp_robber_character) "None" "SnapToTarget" "SnapToTarget" "KeepWorld" false)
      (`self.K2_SetActorRelativeTransform` (`KismetMathLibrary.MakeTransform` (.location (`self.HoldOffset`)) (.rotation (`self.HoldOffset`)) (.scale (`self.HoldOffset`)))))
    (:`Is Not Valid`
      (`self.K2_DetachFromActor` "KeepWorld" "KeepWorld" "KeepWorld")
      (`PrimitiveComponent.SetSimulatePhysics` _mesh true)
      (`PrimitiveComponent.SetCollisionEnabled` _mesh "QueryAndPhysics"))))

(fn `OnRep_HeldBy`
  (`self.ApplyHeldState`))

(fn `Use`
  (params (HitLocation :type "Vector Structure") (HitActor :type "Actor Object Reference"))
  (`KismetSystemLibrary.PrintString` (`KismetStringLibrary.Concat_StrStr` "Used on: " (`KismetSystemLibrary.GetDisplayName` HitActor))))

(fn `UserConstructionScript`
  (`parent.UserConstructionScript`))