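; BP_Cutters is a cutters tool that a robber character can pick up by interacting with it.
; Interact acts only when nothing holds the cutters, casting the interacting player to BP_RobberCharacter and passing itself to Pickup.
; On authority, it then casts HeldBy to the robber and sets HasCutters to true; the ServerInteract branch is empty.
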(event `/Game/OurStuff/Core/InteractionSystem/BPI_Interaction.Interact`
  (params (InteractingPlayer :type "Actor Object Reference") (`ServerInteract?` :type Boolean))
  (if `ServerInteract?`
    _
    (else
      _))
  (if (not (`KismetSystemLibrary.IsValid` (`self.HeldBy`)))
    (bind _asbp_robber_character (cast `/Game/OurStuff/Core/Player/Game/BP_RobberCharacter` InteractingPlayer))
    (`/Game/OurStuff/Core/Player/Game/BP_RobberCharacter.Pickup` _asbp_robber_character self)
    (`/Engine/EditorBlueprintResources/ActorMacros.Switch Has Authority`
      (:`Authority`
        (bind _asbp_robber_character_2 (cast `/Game/OurStuff/Core/Player/Game/BP_RobberCharacter` (`self.HeldBy`)))
        (set `/Game/OurStuff/Core/Player/Game/BP_RobberCharacter.hasCutters` true _asbp_robber_character_2)))))

(fn `UserConstructionScript`
  (`parent.UserConstructionScript`))