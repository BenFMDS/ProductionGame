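; BP_Gabe is the talking NPC Gabe, which players can interact with for a conversation.
; Interact calls TalkToNPC and unlocks an achievement, while GetInteractData returns the prompt text.
; Tick turns the actor's yaw toward a valid PlayerRef, though the nodes here that set that reference are disconnected.
; Legacy behavior-tree dialogue and a shield-based tree swap remain unwired, with comments noting native server-authoritative conversation replaced the old dialogue.
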(event `self.Interact`
  (params (InteractingPlayer :type "Actor Object Reference") (`ServerInteract?` :type Boolean))
  (`DialogueInteractionLibrary.TalkToNPC` self InteractingPlayer)
  (`AchievementSubsystem.UnlockAchievement` (`AchievementBlueprintFunctionLibrary.GetAchievementSubsystem`) "1"))

(event `self.ReceiveTick`
  (params (DeltaSeconds :type "Float (single-precision)"))
  (`self.Player Ref`
    (:`then`
      (`self.Look At Player`))
    (:`else`)))

(event `Look At Player`
  (bind (_returnvalue_roll _returnvalue_pitch _returnvalue_yaw) (`KismetMathLibrary.BreakRotator` (`KismetMathLibrary.FindLookAtRotation` (`SceneComponent.K2_GetComponentLocation` (`self.Mesh`)) (`SceneComponent.K2_GetComponentLocation` (`Character.Mesh` (`self.Player Ref`))))))
  (`self.K2_SetActorRotation` (`KismetMathLibrary.MakeRotator` 0.0 0.0 _returnvalue_yaw)))

(fn `GetInteractData`
  (returns (InteractText :type String))
  (return (`self.Interact Text`)))

(fn `UserConstructionScript`)