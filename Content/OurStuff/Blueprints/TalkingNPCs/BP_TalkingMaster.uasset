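; Base Blueprint for talking exhibit NPCs that can face a player and take part in puzzle quests.
; Tick yaws the actor toward PlayerRef's mesh when valid, though this graph's code that sets PlayerRef is disconnected.
; Puzzle solves pass to C++ for the night director to ready the quest crew-wide.
; Legacy BPCDialogue calls are also disconnected, replaced by native server-authoritative conversation.
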(event `self.ReceiveTick`
  (params (DeltaSeconds :type "Float (single-precision)"))
  (`self.Player Ref`
    (:`then`
      (`self.Look At Player`))
    (:`else`)))

(event `/Game/OurStuff/Core/InteractionSystem/BPI_PuzzleSolver.On Puzzle Solved`
  (params (Puzzle :type "Actor Object Reference") (`Solved By` :type "Pawn Object Reference"))
  ;[1 0.85 0.3] PUZZLE QUESTS: the night director puts an exhibit on a puzzle's Solve Targets when the exhibit's quest is to solve it. This passes the solve to C++ (night director), which readies the quest for the whole crew.
  (`self.HandlePuzzleSolved` Puzzle `Solved By`))

(event `Look At Player`
  (bind (_returnvalue_roll _returnvalue_pitch _returnvalue_yaw) (`KismetMathLibrary.BreakRotator` (`KismetMathLibrary.FindLookAtRotation` (`SceneComponent.K2_GetComponentLocation` (`self.Mesh`)) (`SceneComponent.K2_GetComponentLocation` (`Character.Mesh` (`self.Player Ref`))))))
  (`self.K2_SetActorRotation` (`KismetMathLibrary.MakeRotator` 0.0 0.0 _returnvalue_yaw)))

(fn `UserConstructionScript`)