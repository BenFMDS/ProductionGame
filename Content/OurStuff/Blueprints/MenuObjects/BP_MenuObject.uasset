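; BP_MenuObject is an interactable 3D menu prop with a floating label, configured by a display text, mesh and object type.
; BeginPlay applies the text and mesh, and every Tick rotates the text to face the player camera.
; Interact switches on the object type, either creating and showing a configured widget on non-server interactions or quitting the game.
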(event `self.ReceiveBeginPlay`
  (`parent.ReceiveBeginPlay`)
  (`TextRenderComponent.K2_SetText` (`self.Text`) (`self.DisplayText`))
  (`StaticMeshComponent.SetStaticMesh` (`self.Mesh`) (`self.ObjectMesh`)))

(event `self.ReceiveTick`
  (params (DeltaSeconds :type "Float (single-precision)"))
  (`parent.ReceiveTick` DeltaSeconds)
  (`self.Look at player`))

(event `/Game/OurStuff/Core/InteractionSystem/BPI_Interaction.Interact`
  (params (InteractingPlayer :type "Actor Object Reference") (`ServerInteract?` :type Boolean))
  (switch `/Game/OurStuff/Core/Enums/E_MenuObjectType` (`self.Object Type`)
    (:`NewEnumerator0`
      (if (not `ServerInteract?`)
        (bind _returnvalue (`|CreateWidget` (`self.WidgetToOpen`)))
        (bind _output_get (set `self.MenuRef` _returnvalue))
        (if (not (`Widget.IsInViewport` _output_get))
          (`UserWidget.AddToViewport` (`self.MenuRef`) 0))))
    (:`NewEnumerator1`
      (`KismetSystemLibrary.QuitGame` null "Quit"))))

(fn `Look at player`
  (`SceneComponent.K2_SetWorldRotation` (`self.Text`) (`KismetMathLibrary.FindLookAtRotation` (`SceneComponent.K2_GetComponentLocation` (`self.Text`)) (`SceneComponent.K2_GetComponentLocation` (`PlayerCameraManager.TransformComponent` (`GameplayStatics.GetPlayerCameraManager` 0)))) false false))

(fn `UserConstructionScript`
  (`parent.UserConstructionScript`))