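; BP_ShiftClock is a prop that displays the current day and the time left in the shift.
; Every tick it casts the game state to BP_ReactorGameState and reads CurrentDay and ShiftTimeRemaining.
; It splits the truncated remaining time into minutes and seconds, then writes the formatted day and countdown to TimeText.
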(event `self.ReceiveTick`
  (params (DeltaSeconds :type "Float (single-precision)"))
  (bind _asbp_reactor_game_state (cast `/Game/OurStuff/Core/Player/Game/BP_ReactorGameState` (`GameplayStatics.GetGameState`)))
  (bind _returnvalue (`KismetMathLibrary.FTrunc` (`/Game/OurStuff/Core/Player/Game/BP_ReactorGameState.ShiftTimeRemaining` _asbp_reactor_game_state)))
  (`TextRenderComponent.K2_SetText` (`self.TimeText`) (`|FormatText` "DAY {day}  {min}:{sec}" (`KismetTextLibrary.Conv_IntToText` (`/Game/OurStuff/Core/Player/Game/BP_ReactorGameState.CurrentDay` _asbp_reactor_game_state)) (/ _returnvalue 60) (`KismetTextLibrary.Conv_IntToText` (mod _returnvalue 60) false true 2))))

(fn `UserConstructionScript`)