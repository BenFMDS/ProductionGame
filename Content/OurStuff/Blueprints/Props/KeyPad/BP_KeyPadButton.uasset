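; BP_KeyPadButton is a single digit button that feeds input to a keypad.
; The construction script writes its Digit to the DigitText component as the visible label.
; On Interact it waits briefly, then passes the digit to the referenced KeyPad through EnterDigit if that reference is valid.
; The ServerInteract branch has no logic on either side.
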(event `/Game/OurStuff/Core/InteractionSystem/BPI_Interaction.Interact`
  (params (InteractingPlayer :type "Actor Object Reference") (`ServerInteract?` :type Boolean))
  (bind _keypad (`self.KeyPad`))
  (`KismetSystemLibrary.Delay` 0.1)
  (if `ServerInteract?`
    _
    (else
      _))
  (`/Engine/EditorBlueprintResources/StandardMacros.IsValid` _keypad
    (:`Is Valid`
      (`/Game/OurStuff/Blueprints/Props/KeyPad/BP_KeyPadDoor.EnterDigit` _keypad (`self.Digit`)))))

(fn `UserConstructionScript`
  (`parent.UserConstructionScript`)
  (`TextRenderComponent.K2_SetText` (`self.DigitText`) (`KismetTextLibrary.Conv_IntToText` (`self.Digit`))))