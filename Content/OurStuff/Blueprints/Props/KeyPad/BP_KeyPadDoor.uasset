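; Keypad-locked sliding door whose four-digit code is picked from a per-day list using the reactor game state's current day.
; The server validates entered digits, clearing a wrong entry or opening the door on a match.
; RepNotify on entry, open and jammed states drives the display and door on clients, with the server calling the same handlers.
; A timeline slides the mesh, halting while jammed and resuming once cleared.
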(event `self.ReceiveBeginPlay`
  (`KismetSystemLibrary.Delay` 0.3)
  (if (`self.HasAuthority`)
    (bind _asbp_reactor_game_state (cast `/Game/OurStuff/Core/Player/Game/BP_ReactorGameState` (`GameplayStatics.GetGameState`))
      (:`then`
        (set `self.TodaysCode` (`|GetArrayItem` (`self.CodesPerDay`) (mod (- (`/Game/OurStuff/Core/Player/Game/BP_ReactorGameState.CurrentDay` _asbp_reactor_game_state) 1) (`KismetArrayLibrary.Array_Length` (`self.CodesPerDay`))))))
      (:`CastFailed`
        (`KismetSystemLibrary.PrintString` "Cast Failed")))))

(event `DoorMotion`
  (if (`self.Open`)
    (bind (_direction _doorslide) (`Timeline|DoorSlide` :!label _label)
      (:`Update`
        (if (`self.Jammed`)
          (goto _label :!via `Stop`)
          (else
            (`SceneComponent.K2_SetRelativeLocation` (`self.DoorMesh`) (`KismetMathLibrary.VLerp` (0.0 0.0 0.0) (`self.OpenOffset`) _doorslide) false false)))))
    (else
      (goto _label :!via `Reverse`))))

(fn `ApplyDoorState`
  (`self.DoorMotion`))

(fn `EnterDigit`
  (params (Digit :type Integer))
  (bind _currententry (`self.CurrentEntry`))
  (if (`self.HasAuthority`)
    (if (not (`self.Open`))
      (set `self.CurrentEntry` (`KismetStringLibrary.Concat_StrStr` (`self.CurrentEntry`) (`KismetStringLibrary.Conv_IntToString` Digit)))
      (`self.RefreshDisplay`)
      (if (>= (`KismetStringLibrary.Len` _currententry) 4)
        (if (`KismetStringLibrary.EqualEqual_StrStr` _currententry (`self.TodaysCode`))
          (set `self.Open` true)
          (`self.ApplyDoorState`)
          (else
            (set `self.CurrentEntry` "")
            (`self.RefreshDisplay`)))))))

(fn `JamStateChanged`
  (if (not (`self.Jammed`))
    (`self.DoorMotion`)))

(fn `OnRep_CurrentEntry`
  (`self.RefreshDisplay`))

(fn `OnRep_Jammed`
  (`self.JamStateChanged`))

(fn `OnRep_Open`
  (`self.ApplyDoorState`))

(fn `RefreshDisplay`
  (`TextRenderComponent.K2_SetText` (`self.EntryDisplay`) (`KismetTextLibrary.Conv_StringToText` (`self.CurrentEntry`))))

(fn `SetJammed`
  (params (Jammed :type Boolean))
  (if (`self.HasAuthority`)
    (set `self.Jammed` Jammed)
    (`self.JamStateChanged`)))

(fn `UserConstructionScript`)