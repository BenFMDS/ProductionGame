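; BP_LootBase is a base physics loot prop with a name, value and weight, which players grab and carry for delivery.
; Construction builds the prompt, overrides mesh mass and ignores Pawn collision; Interact starts BPC_PhysicsCarry on authority.
; Holder changes split weight among carriers, setting each one's carry speed to that share over SlowWeight, clamped.
; CanBeDelivered requires loot be undelivered and unheld.
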(event `self.ReceiveBeginPlay`
  (`parent.ReceiveBeginPlay`))

(event `/Game/OurStuff/Core/InteractionSystem/BPI_Interaction.Interact`
  (params (InteractingPlayer :type "Actor Object Reference") (`ServerInteract?` :type Boolean))
  (bind _returnvalue (`self.GetComponentByClass` InteractingPlayer "/Game/OurStuff/Core/InteractionSystem/BPC_PhysicsCarry.BPC_PhysicsCarry_C"))
  (`/Engine/EditorBlueprintResources/ActorMacros.Switch Has Authority`
    (:`Authority`
      (`/Engine/EditorBlueprintResources/StandardMacros.IsValid` _returnvalue
        (:`Is Valid`
          (`/Game/OurStuff/Core/InteractionSystem/BPC_PhysicsCarry.StartCarry` _returnvalue self))))))

(fn `AddHolder`
  (params (Holder :type "Actor Object Reference"))
  (`KismetArrayLibrary.Array_AddUnique` (`self.Holders`) Holder)
  (`self.UpdateHolderSpeeds`))

(fn `CanBeDelivered`
  (returns (Result :type Boolean))
  ; Not already counted and Nobody is holding it
  (return (and (not (`self.Delivered`)) (not (`KismetSystemLibrary.IsValid` (`self.HeldBy`))))))

(fn `RemoveHolder`
  (params (Holder :type "Actor Object Reference"))
  (`KismetArrayLibrary.Array_RemoveItem` (`self.Holders`) Holder)
  (`self.UpdateHolderSpeeds`))

(fn `UpdateHolderSpeeds`
  (locals (Share :type "Float (double-precision)") (Multiplier :type "Float (double-precision)"))
  (set `local.Share` (/ (`self.Weight`) (`KismetMathLibrary.FMax` 1.0 (`KismetMathLibrary.Conv_IntToDouble` (`KismetArrayLibrary.Array_Length` (`self.Holders`))))))
  (set `local.Multiplier` (`KismetMathLibrary.FClamp` (/ (`local.Share`) (`self.SlowWeight`)) (`self.MinSpeed`)))
  (for _array_element (`self.Holders`)
    (bind _returnvalue (`self.GetComponentByClass` _array_element "/Game/OurStuff/Core/InteractionSystem/BPC_PhysicsCarry.BPC_PhysicsCarry_C"))
    (`/Engine/EditorBlueprintResources/StandardMacros.IsValid` _returnvalue
      (:`Is Valid`
        (`/Game/OurStuff/Core/InteractionSystem/BPC_PhysicsCarry.SetCarrySpeed` _returnvalue (`local.Multiplier`))))))

(fn `UserConstructionScript`
  (`parent.UserConstructionScript`)
  (set `self.Interact Text` (`KismetTextLibrary.Conv_TextToString` (`|FormatText` "Grab {Name} (${Value})" (`self.LootName`) (`self.LootValue`))))
  (`PrimitiveComponent.SetMassOverrideInKg` (`self.Mesh`) "None" (`self.Weight`) true)
  (`PrimitiveComponent.SetCollisionResponseToChannel` (`self.Mesh`) "ECC_Pawn" "ECR_Ignore"))