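; Loot drop zone that turns delivered BP_LootBase props into take for the robbers while the zone is Active.
; The server checks DropBox on overlap (a tick later) and on a looping timer, feeding both into TryDeliver.
; TryDeliver credits the game state, releases carriers, destroys the loot and plays a cash sound.
; The construction script and Active's RepNotify show or hide the cube and labels.
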(event `self.ReceiveBeginPlay`
  (`/Engine/EditorBlueprintResources/ActorMacros.Switch Has Authority`
    (:`Authority`
      (`KismetSystemLibrary.K2_SetTimerDelegate` (delegate `CheckZone`) 0.5 true))))

(event `CheckZone`
  (for _array_element (`PrimitiveComponent.GetOverlappingActors` (`self.DropBox`) "/Game/OurStuff/Blueprints/Props/Loot/BP_LootBase.BP_LootBase_C")
    (bind _asbp_loot_base (cast `/Game/OurStuff/Blueprints/Props/Loot/BP_LootBase` _array_element))
    (`self.TryDeliver` _asbp_loot_base)))

(event `self.DropBox.OnComponentBeginOverlap`
  (params (OverlappedComponent :type "PrimitiveComponent Object Reference") (OtherActor :type "Actor Object Reference") (OtherComp :type "PrimitiveComponent Object Reference") (OtherBodyIndex :type Integer) (bFromSweep :type Boolean) (SweepResult :type "HitResult Structure (by ref)"))
  (`/Engine/EditorBlueprintResources/ActorMacros.Switch Has Authority`
    (:`Authority`
      (`KismetSystemLibrary.DelayUntilNextTick`)
      (bind _asbp_loot_base (cast `/Game/OurStuff/Blueprints/Props/Loot/BP_LootBase` OtherActor))
      (`self.TryDeliver` _asbp_loot_base))))

(fn `OnRep_Active`
  (bind _returnvalue (not (`self.Active`)))
  (`SceneComponent.SetHiddenInGame` (`self.Cube`) _returnvalue false)
  (`SceneComponent.SetHiddenInGame` (`self.TextRender`) _returnvalue false)
  (`SceneComponent.SetHiddenInGame` (`self.TextRender1`) _returnvalue false))

(fn `TryDeliver`
  (params (Loot :type "/Game/OurStuff/Blueprints/Props/Loot/BP_LootBase Object Reference"))
  (locals (HoldersCopy :type "Array of Actor Object Reference"))
  (if (and (`KismetSystemLibrary.IsValid` Loot) (`self.HasAuthority`) (`/Game/OurStuff/Blueprints/Props/Loot/BP_LootBase.CanBeDelivered` Loot) (`self.Active`))
    (set `/Game/OurStuff/Blueprints/Props/Loot/BP_LootBase.Delivered` true Loot)
    (bind _asbp_robber_game_state (cast `/Game/OurStuff/Core/Player/Game/BP_RobberGameState` (`GameplayStatics.GetGameState`)))
    (`/Game/OurStuff/Core/Player/Game/BP_RobberGameState.AddToTake` _asbp_robber_game_state (`/Game/OurStuff/Blueprints/Props/Loot/BP_LootBase.LootValue` Loot))
    (`/Game/OurStuff/Core/Player/Game/BP_RobberGameState.LootDelivered` _asbp_robber_game_state (`/Game/OurStuff/Blueprints/Props/Loot/BP_LootBase.LootName` Loot) (`/Game/OurStuff/Blueprints/Props/Loot/BP_LootBase.LootValue` Loot))
    (bind _output_get (set `local.HoldersCopy` (`/Game/OurStuff/Blueprints/Props/Loot/BP_LootBase.Holders` Loot)))
    (for _array_element _output_get
      (bind _returnvalue (`self.GetComponentByClass` _array_element "/Game/OurStuff/Core/InteractionSystem/BPC_PhysicsCarry.BPC_PhysicsCarry_C"))
      (`/Engine/EditorBlueprintResources/StandardMacros.IsValid` _returnvalue
        (:`Is Valid`
          (`/Game/OurStuff/Core/InteractionSystem/BPC_PhysicsCarry.StopCarry` _returnvalue))))
    (`self.K2_DestroyActor` Loot)
    (`GameplayStatics.PlaySoundAtLocation` "/Game/OurStuff/Assets/Audio/SW_Cash.SW_Cash" (`self.K2_GetActorLocation`) (struct) 1.0 1.0 0.0 null null null null)))

(fn `UserConstructionScript`
  (bind _returnvalue (not (`self.Active`)))
  (`SceneComponent.SetHiddenInGame` (`self.Cube`) _returnvalue false)
  (`SceneComponent.SetHiddenInGame` (`self.TextRender`) _returnvalue false)
  (`SceneComponent.SetHiddenInGame` (`self.TextRender1`) _returnvalue false))