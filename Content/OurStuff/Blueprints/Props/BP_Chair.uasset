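; Chair prop that seats a reactor character when a player interacts with it.
; Interact proceeds only if no valid Occupant is set, casts the player to BP_ReactorCharacter, stores it as Occupant and calls its SitDown with the chair.
; The ServerInteract flag does not change the behavior, and nothing in this graph clears Occupant.
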(event `/Game/OurStuff/Core/InteractionSystem/BPI_Interaction.Interact`
  (params (InteractingPlayer :type "Actor Object Reference") (`ServerInteract?` :type Boolean))
  (if `ServerInteract?`
    _
    (else
      _))
  (`/Engine/EditorBlueprintResources/StandardMacros.IsValid` (`self.Occupant`)
    (:`Is Not Valid`
      (bind _asbp_reactor_character (cast `/Game/OurStuff/Core/Player/Game/BP_ReactorCharacter` InteractingPlayer))
      (set `self.Occupant` _asbp_reactor_character)
      (`/Game/OurStuff/Core/Player/Game/BP_ReactorCharacter.SitDown` _asbp_reactor_character self))))

(fn `UserConstructionScript`
  (`parent.UserConstructionScript`))