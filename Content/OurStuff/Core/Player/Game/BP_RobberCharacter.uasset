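; First-person robber player character for a multiplayer stealth game with guards, handling crouch, footsteps, proximity voice chat and a locally spawned map attached to the camera.
; Held items are picked up, dropped or thrown under server authority, and used through a camera box trace.
; A looping timer drives adaptive music from the highest alert state of guards targeting this robber.
; Overlapping lit areas are counted to set player visibility.
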(event `PlayFadeForwardServer`
  ; Transition
  (`self.PlayFadeForward`))

(event `PlayFadeBackwardsServer`
  ; Transition
  (`self.PlayFadeBackwards`))

(event `PlayFadeForward`
  ; Transition
  (bind (_direction _fadevalue) (`Timeline|Timeline` :!via `PlayFromStart` :!label _label)
    (:`Update`
      (`MaterialInstanceDynamic.SetScalarParameterValue` (`self.Fade Material`) "Fade" _fadevalue))))

(event `PlayFadeBackwards`
  ; Transition
  (goto _label :!via `Reverse`))

(event `self.ReceiveTick`
  (params (DeltaSeconds :type "Float (single-precision)"))
  (bind _footstep (`self.Footstep`))
  (bind _returnvalue (`AudioComponent.IsPlaying` _footstep))
  (if (and (> (`KismetMathLibrary.VSizeXY` (`SceneComponent.GetComponentVelocity` (`self.CapsuleComponent`))) 1.0) (`NavMovementComponent.IsMovingOnGround` (`self.CharacterMovement`)))
    (if (not _returnvalue)
      (`AudioComponent.FadeIn` _footstep 0.1 1.0 0.0 "Linear"))
    (elif _returnvalue
      (`AudioComponent.FadeOut` _footstep 0.1 0.0 "Linear"))))

(event `self.ReceiveBeginPlay`
  (`self.StartVoiceChat`)
  ; Mesh Base Z for crouch
  (set `self.MeshBaseZ` (.z (`SceneComponent.RelativeLocation` (`self.FirstPersonMesh`))))
  ; Update Music
  (`KismetSystemLibrary.K2_SetTimerDelegate` (`|CreateDelegate` :!event `UpdateMusic`) 0.25 true))

(event `self.Primary Thumbstick`
  (params (Axis :type "Vector2D Structure"))
  ; Touch Inputs for First Person Character
  (`self.DoMove` Axis_X Axis_Y))

(event `StartVoiceChat`
  (bind _playerstate (`self.PlayerState`))
  ; Voice Chat
  (bind _returnvalue (`AddComponent|NODE_AddVOIPTalker-0`))
  (set `self.VOIPRef` _returnvalue)
  (`/Engine/EditorBlueprintResources/StandardMacros.IsValid` _playerstate :!label _label_2
    (:`Is Valid`
      (`VOIPTalker.RegisterWithPlayerState` (`self.VOIPRef`) _playerstate)
      (`VOIPStatics.SetMicThreshold` -1.0)
      (set `VOIPTalker.Settings` (make `VoiceSettings` (`self.FirstPersonCameraComponent`) "/Game/OurStuff/Audio/SA_VoiceChat.SA_VoiceChat") (`self.VOIPRef`))
      (`KismetSystemLibrary.ExecuteConsoleCommand` "ToggleSpeaking 1" null)
      (if (`self.IsLocallyControlled`)
        _))
    (:`Is Not Valid`
      (`KismetSystemLibrary.Delay` 0.2)
      (goto _label_2))))

(event `self.Secondary Thumbstick`
  (params (Axis :type "Vector2D Structure"))
  ; Touch Inputs for First Person Character
  (`self.DoAim` Axis_X Axis_Y))

(event `Key|One`
  (params (Key :type "Key Structure"))
  (:`Pressed`
    (set `self.HasShield?` true)))

(event `self.Touch Jump Start`
  ; Touch Inputs for First Person Character
  (`self.DoJumpStart`))

(event `Key|V`
  (params (Key :type "Key Structure"))
  ; Voice Chat
  (:`Pressed`
    (`KismetSystemLibrary.ExecuteConsoleCommand` "OSS.VoiceLoopback 1" null))
  (:`Released`
    (`KismetSystemLibrary.ExecuteConsoleCommand` "ToggleSpeaking 0" null)))

(event `self.Touch Jump End`
  ; Touch Inputs for First Person Character
  (`self.DoJumpEnd`))

(event `EnhancedInput|/Game/Input/Actions/IA_Crouch`
  (params (ActionValue :type Boolean) (ElapsedSeconds :type "Float (double-precision)") (TriggeredSeconds :type "Float (double-precision)") (InputAction :type "InputAction Object Reference" :default "/Game/Input/Actions/IA_Crouch.IA_Crouch"))
  ; Crouch
  (:`Started`
    (`self.Crouch`))
  (:`Completed`
    (`self.UnCrouch`)))

(event `Server_DropHeld`
  (params (Impulse :type "Float (double-precision)"))
  ; Comment
  (`self.DropHeld` Impulse))

(event `EnhancedInput|/Game/Input/Actions/IA_Drop`
  (params (ActionValue :type Boolean) (ElapsedSeconds :type "Float (double-precision)") (TriggeredSeconds :type "Float (double-precision)") (InputAction :type "InputAction Object Reference" :default "/Game/Input/Actions/IA_Drop.IA_Drop"))
  ; Comment
  (:`Started`
    (`self.Server_DropHeld` 0.0)))

(event `self.K2_OnStartCrouch`
  (params (HalfHeightAdjust :type "Float (single-precision)") (ScaledHalfHeightAdjust :type "Float (single-precision)"))
  (bind _firstpersonmesh (`self.FirstPersonMesh`))
  ; Crouch
  (bind (_direction _alpha) (`Timeline|CrouchView` :!label _label_3)
    (:`Update`
      (`SceneComponent.K2_SetRelativeLocation` _firstpersonmesh (`KismetMathLibrary.MakeVector` (.x (`SceneComponent.RelativeLocation` _firstpersonmesh)) (.y (`SceneComponent.RelativeLocation` _firstpersonmesh)) (- (`self.MeshBaseZ`) (* (`self.CrouchViewDrop`) _alpha))) false false))))

(event `EnhancedInput|/Game/Input/Actions/IA_Throw`
  (params (ActionValue :type Boolean) (ElapsedSeconds :type "Float (double-precision)") (TriggeredSeconds :type "Float (double-precision)") (InputAction :type "InputAction Object Reference" :default "/Game/Input/Actions/IA_Throw.IA_Throw"))
  (bind _helditem (`self.HeldItem`))
  ; Comment
  (:`Started`
    (`/Engine/EditorBlueprintResources/StandardMacros.IsValid` _helditem
      (:`Is Valid`
        (`self.Server_DropHeld` (`/Game/OurStuff/Blueprints/Tools/BP_Holdable.ThrowStrength` _helditem))))))

(event `self.K2_OnEndCrouch`
  (params (HalfHeightAdjust :type "Float (single-precision)") (ScaledHalfHeightAdjust :type "Float (single-precision)"))
  ; Crouch
  (goto _label_3 :!via `Reverse`))

(event `EnhancedInput|/Game/Input/Actions/IA_Use`
  (params (ActionValue :type Boolean) (ElapsedSeconds :type "Float (double-precision)") (TriggeredSeconds :type "Float (double-precision)") (InputAction :type "InputAction Object Reference" :default "/Game/Input/Actions/IA_Use.IA_Use"))
  ; Comment
  (:`Started`
    (`self.Server_UseHeld`)))

(event `Server_UseHeld`
  (bind _helditem (`self.HeldItem`))
  (bind _returnvalue (`SceneComponent.K2_GetComponentLocation` (`self.FirstPersonCameraComponent`)))
  ; Comment
  (`/Engine/EditorBlueprintResources/StandardMacros.IsValid` _helditem
    (:`Is Valid`
      (bind _outhits (`KismetSystemLibrary.BoxTraceMulti` _returnvalue (+ _returnvalue (* (`KismetMathLibrary.GetForwardVector` (`self.GetControlRotation`)) 400.0)) (3.0 3.0 3.0) (struct) "TraceTypeQuery1" false (`|MakeArray` _helditem :!type "Actor Object Reference")))
      (for _array_element _outhits
        (bind (_bblockinghit _binitialoverlap _time _distance _location _impactpoint _normal _impactnormal _physmat _hitactor) (`GameplayStatics.BreakHitResult` _array_element))
        (`/Game/OurStuff/Blueprints/Tools/BP_Holdable.Use` (`self.HeldItem`) _location _hitactor _impactpoint)))))

(event `UpdateMusic`
  (bind _alert (`self.Alert`))
  ; Play Music: Depending on guard state
  (if (`self.IsLocallyControlled`)
    (if (not (`self.MusicStarted`))
      (`AudioComponent.Play` (`self.Music`) 0.0)
      (set `self.MusicStarted` true))
    (set `self.Alert` 0.0)
    (bind _outactors (`GameplayStatics.GetAllActorsOfClass` "/Game/OurStuff/Blueprints/Guard/BP_Guard.BP_Guard_C"))
    (for _array_element _outactors
      (if (== (`/Game/OurStuff/Blueprints/Guard/BP_Guard.TargetRobber` _array_element) self)
        (set `self.Alert` (`KismetMathLibrary.FMax` (`self.Alert`) (select `/Game/OurStuff/Blueprints/Guard/E_GuardState` (`/Game/OurStuff/Blueprints/Guard/BP_Guard.GuardState` _array_element) :`NewEnumerator1` 0.3 :`NewEnumerator2` 0.6 :`NewEnumerator3` 1.0)))))
    (if (!= (`self.Alert`) (`self.CurrentAlert`))
      (`AudioParameterControllerInterface.SetFloatParameter` (`self.Music`) "EnemyAlert" _alert)
      (set `self.CurrentAlert` _alert))))

(event `self.ReceiveControllerChanged`
  (params (OldController :type "Controller Object Reference") (NewController :type "Controller Object Reference"))
  ; Spawn and Attach the Map
  (bind _asbp_robber_controller (cast `/Game/OurStuff/Core/Player/Game/BP_RobberController` (`self.GetController`)))
  (`WidgetBlueprintLibrary.SetInputMode_GameOnly` _asbp_robber_controller)
  (if (and (`self.IsLocallyControlled`) (not (`KismetSystemLibrary.IsValid` (`self.HeldMap`))))
    (bind _returnvalue (`|SpawnActorFromClass` "/Game/OurStuff/Blueprints/Map/BP_HeldMap.BP_HeldMap_C" (`SceneComponent.K2_GetComponentToWorld` (`self.FirstPersonCameraComponent`)) "AlwaysSpawn" "MultiplyWithRoot" self null))
    (bind _output_get (set `self.HeldMap` _returnvalue))
    (`self.K2_AttachToComponent` _output_get (`self.FirstPersonCameraComponent`) "None" "SnapToTarget" "SnapToTarget" "SnapToTarget" false)))

(event `self.ReceiveEndPlay`
  (params (EndPlayReason :type "EEndPlayReason Enum" :default "Destroyed"))
  (bind _heldmap (`self.HeldMap`))
  ; Spawn and Attach the Map
  (`/Engine/EditorBlueprintResources/StandardMacros.IsValid` _heldmap
    (:`Is Valid`
      (`self.K2_DestroyActor` _heldmap))))

(fn `DropHeld`
  (params (Impulse :type "Float (double-precision)"))
  (locals (Item :type "/Game/OurStuff/Blueprints/Tools/BP_Holdable Object Reference"))
  (bind _helditem (`self.HeldItem`))
  (if (`self.HasAuthority`)
    (`/Engine/EditorBlueprintResources/StandardMacros.IsValid` _helditem
      (:`Is Valid`
        (bind _output_get (set `local.Item` _helditem))
        (set `/Game/OurStuff/Blueprints/Tools/BP_Holdable.HeldBy` null _output_get)
        (`/Game/OurStuff/Blueprints/Tools/BP_Holdable.ApplyHeldState` _output_get)
        (if (> Impulse 0.0)
          (`PrimitiveComponent.AddImpulse` (`/Game/OurStuff/Blueprints/BP_InteractMaster.Mesh` _output_get) (* (`SceneComponent.GetForwardVector` (`self.FirstPersonCameraComponent`)) Impulse) "None" true))
        (`self.SetOwner` _output_get null)
        (set `self.HeldItem` null)
        (set `self.hasCutters` false)))))

(fn `EnterLitArea`
  (bind _output_get (set `self.LitLightCount` (+ (`self.LitLightCount`) 1)))
  (set `self.PlayerVisable` (> (`KismetMathLibrary.Clamp` _output_get 0 999) 0))
  (`KismetSystemLibrary.PrintString` "Player Visable"))

(fn `ExitLitArea`
  (bind _output_get (set `self.LitLightCount` (- (`self.LitLightCount`) 1)))
  (set `self.PlayerVisable` (> (`KismetMathLibrary.Clamp` _output_get 0 999) 0))
  (`KismetSystemLibrary.PrintString` "Player Not Visable"))

(fn `Pickup`
  (params (Item :type "/Game/OurStuff/Blueprints/Tools/BP_Holdable Object Reference"))
  (if (`self.HasAuthority`)
    (`/Engine/EditorBlueprintResources/StandardMacros.IsValid` (`self.HeldItem`)
      (:`Is Valid`
        (`self.DropHeld` 0.0))
      (:`Is Not Valid`
        _))
    (bind _output_get (set `self.HeldItem` Item))
    (`self.SetOwner` _output_get self)
    (set `/Game/OurStuff/Blueprints/Tools/BP_Holdable.HeldBy` self _output_get)
    (`/Game/OurStuff/Blueprints/Tools/BP_Holdable.ApplyHeldState` _output_get)))

(fn `UserConstructionScript`)