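; Game state for the robber game that tracks the team's take, shared debt, cash and night count.
; On BeginPlay the server loads these totals from the game instance's debt save and listens for stage changes that flag the gem as taken or trigger payout.
; The once-only, authority-checked payout adds any gem value, puts a capped share toward debt, sets cash to the remainder, advances the night and saves.
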(event `self.ReceiveBeginPlay`
  (`/Engine/EditorBlueprintResources/ActorMacros.Switch Has Authority`
    (:`Authority`
      (bind _asbp_game_instance (cast `/Game/OurStuff/Core/Player/Game/BP_GameInstance` (`GameplayStatics.GetGameInstance`)))
      (`/Game/OurStuff/Core/Player/Game/BP_GameInstance.GetDebtSave` _asbp_game_instance)
      (bind _debtsave (`/Game/OurStuff/Core/Player/Game/BP_GameInstance.DebtSave` _asbp_game_instance))
      (set `self.DebtRemaining` (`/Game/OurStuff/Core/Player/Game/DebtSystem/BP_DebtSave.DebtRemaining` _debtsave))
      (set `self.Cash` (`/Game/OurStuff/Core/Player/Game/DebtSystem/BP_DebtSave.Cash` _debtsave))
      (set `self.Night` (`/Game/OurStuff/Core/Player/Game/DebtSystem/BP_DebtSave.Night` _debtsave))
      (add `self.OnGameStageChanged` (`|CreateDelegate` :!event `HandleStageChanged`)))))

(event `HandleStageChanged` :!signature `self.OnGameStageChanged`
  (params (NewGameStage :type Byte))
  (`|ExecutionSequence`
    (:`then_0`
      (if (== NewGameStage 3)
        (set `self.GemTaken` true)))
    (:`then_1`
      (if (== NewGameStage 6)
        (`self.ApplyNightPayout`)))))

(event `DebugAddTake`
  (params (Amount :type Integer))
  ; Debug
  (`/Engine/EditorBlueprintResources/ActorMacros.Switch Has Authority`
    (:`Authority`
      (`self.AddToTake` Amount))))

(event `DebugPayout`
  ; Debug
  (set `self.PaidOut` false)
  (`self.ApplyNightPayout`))

(event `LootDelivered`
  (params (LootName :type Text) (Value :type Integer)))

(fn `AddToTake`
  (params (Amount :type Integer))
  (if (and (> Amount 0) (`self.HasAuthority`))
    (set `self.TeamTake` (+ (`self.TeamTake`) Amount))))

(fn `ApplyNightPayout`
  (locals (Take :type Integer) (ToDebt :type Integer))
  (if (and (`self.HasAuthority`) (!= (`self.PaidOut`) true))
    (set `self.PaidOut` true)
    (bind _output_get (set `local.Take` (+ (`self.TeamTake`) (`KismetMathLibrary.SelectInt` 0 (`self.GemValue`) (`self.GemTaken`)))))
    (bind _output_get_2 (set `local.ToDebt` (`KismetMathLibrary.Min` (`KismetMathLibrary.Round` (* _output_get (`self.DebtShare`))) (`self.DebtRemaining`))))
    (set `self.DebtRemaining` (- (`self.DebtRemaining`) _output_get_2))
    (set `self.Cash` (- (`local.Take`) (`local.ToDebt`)))
    (bind _result (`/Engine/EditorBlueprintResources/StandardMacros.IncrementInt` (`self.Night`))
      (:`  `
        (set `self.Night` _result)
        (set `self.TeamTake` 0)
        (bind _asbp_game_instance (cast `/Game/OurStuff/Core/Player/Game/BP_GameInstance` (`GameplayStatics.GetGameInstance`)))
        (bind _saveobject (`/Game/OurStuff/Core/Player/Game/BP_GameInstance.GetDebtSave` _asbp_game_instance))
        (set `/Game/OurStuff/Core/Player/Game/DebtSystem/BP_DebtSave.DebtRemaining` (`self.DebtRemaining`) _saveobject)
        (set `/Game/OurStuff/Core/Player/Game/DebtSystem/BP_DebtSave.Cash` (`self.Cash`) _saveobject)
        (set `/Game/OurStuff/Core/Player/Game/DebtSystem/BP_DebtSave.Night` (`self.Night`) _saveobject)
        (`/Game/OurStuff/Core/Player/Game/BP_GameInstance.SaveDebt` _asbp_game_instance)
        (if (<= (`self.DebtRemaining`) 0)
          (`KismetSystemLibrary.PrintString` "Debt Cleared" true true (struct :`R` 0.263652 :`G` 1.0 :`A` 1.0)))))))

(fn `OnRep_DebtRemaining`)

(fn `UserConstructionScript`)