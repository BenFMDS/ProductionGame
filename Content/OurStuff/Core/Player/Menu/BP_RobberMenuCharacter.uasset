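; First-person robber character, named for menu use, that sets up positional voice chat on BeginPlay and forwards touch controls to move, aim and jump functions.
; Voice setup creates a VOIP talker, polls until PlayerState is valid, then registers it with camera attachment and attenuation and switches speaking on.
; Pressing V enables voice loopback, while releasing it stops speaking; the 1 key sets the shield flag.
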(event `self.Primary Thumbstick`
  (params (Axis :type "Vector2D Structure"))
  ; Touch Inputs for First Person Character
  (`self.DoMove` Axis_X Axis_Y))

(event `self.Secondary Thumbstick`
  (params (Axis :type "Vector2D Structure"))
  ; Touch Inputs for First Person Character
  (`self.DoAim` Axis_X Axis_Y))

(event `self.Touch Jump Start`
  ; Touch Inputs for First Person Character
  (`self.DoJumpStart`))

(event `self.Touch Jump End`
  ; Touch Inputs for First Person Character
  (`self.DoJumpEnd`))

(event `self.ReceiveBeginPlay`
  (`self.StartVoiceChat`))

(event `StartVoiceChat`
  (bind _playerstate (`self.PlayerState`))
  (bind _returnvalue (`AddComponent|NODE_AddVOIPTalker-0`))
  (set `self.VOIPRef` _returnvalue)
  (`/Engine/EditorBlueprintResources/StandardMacros.IsValid` _playerstate :!label _label
    (:`Is Valid`
      (`VOIPTalker.RegisterWithPlayerState` (`self.VOIPRef`) _playerstate)
      (`VOIPStatics.SetMicThreshold` -1.0)
      (set `VOIPTalker.Settings` (make `VoiceSettings` (`self.FirstPersonCameraComponent`) "/Game/OurStuff/Audio/SA_VoiceChat.SA_VoiceChat") (`self.VOIPRef`))
      (`KismetSystemLibrary.ExecuteConsoleCommand` "ToggleSpeaking 1" null)
      (if (`self.IsLocallyControlled`)
        _))
    (:`Is Not Valid`
      (`KismetSystemLibrary.Delay` 0.2)
      (goto _label))))

(event `Key|V`
  (params (Key :type "Key Structure"))
  (:`Pressed`
    (`KismetSystemLibrary.ExecuteConsoleCommand` "OSS.VoiceLoopback 1" null))
  (:`Released`
    (`KismetSystemLibrary.ExecuteConsoleCommand` "ToggleSpeaking 0" null)))

(event `Key|One`
  (params (Key :type "Key Structure"))
  (:`Pressed`
    (set `self.HasShield?` true)))

(fn `UserConstructionScript`)