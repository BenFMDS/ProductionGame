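; Component on the robber pawn that lets it carry, drop and throw physics loot, with the server in authority.
; A server-created physics handle grabs loot at the traced point and follows the view, dropping it if that point strays too far.
; Loot within the lift limit keeps its yaw-relative rotation, while heavier loot is grabbed by location only.
; Loot tracks its holders, and a RepNotify speed multiplier adjusts movement, resetting on release.
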(event `self.ReceiveTick`
  (params (DeltaSeconds :type "Float (single-precision)"))
  (bind (_outlocation _outrotation) (`Actor.GetActorEyesViewPoint` (`self.OwnerPawn`)))
  (bind _returnvalue (`Actor.HasAuthority` (`self.GetOwner`)))
  (bind _returnvalue_2 (+ _outlocation (- (* (`KismetMathLibrary.GetForwardVector` _outrotation) (`self.HoldDistance`)) (* (`KismetMathLibrary.GetUpVector` _outrotation) (`self.HoldDrop`)))))
  (if (and _returnvalue (`KismetSystemLibrary.IsValid` (`self.CarriedLoot`)))
    (if (`self.HoldUpright`)
      (`PhysicsHandleComponent.SetTargetLocationAndRotation` (`self.Handle`) _returnvalue_2 (`KismetMathLibrary.ComposeRotators` (`self.HoldRotOffset`) (`KismetMathLibrary.MakeRotator` 0.0 0.0 (.yaw _outrotation))))
      (else
        (`PhysicsHandleComponent.SetTargetLocation` (`self.Handle`) _returnvalue_2)))
    (if (> (`KismetMathLibrary.Vector_Distance` (`KismetMathLibrary.TransformLocation` (`SceneComponent.K2_GetComponentToWorld` (`/Game/OurStuff/Blueprints/BP_InteractMaster.Mesh` (`self.CarriedLoot`))) (`self.GrabOffsetLocal`)) _returnvalue_2) (`self.BreakDistance`))
      (`self.StopCarry`))
    (elif (and _returnvalue (!= (`self.SpeedMultiplier`) 1.0))
      (`self.SetCarrySpeed` 1.0)
      (set `self.CarriedLoot` null))))

(event `self.ReceiveBeginPlay`
  (bind _returnvalue (`self.GetOwner`))
  (bind _aspawn (cast `Pawn` _returnvalue))
  (bind _output_get (set `self.OwnerPawn` _aspawn))
  (bind _asbp_robber_character (cast `/Game/OurStuff/Core/Player/Game/BP_RobberCharacter` _output_get))
  (bind _charactermovement (`Character.CharacterMovement` _asbp_robber_character))
  (set `self.BaseWalkSpeed` (`CharacterMovementComponent.MaxWalkSpeed` _charactermovement))
  (set `self.BaseCrouchSpeed` (`CharacterMovementComponent.MaxWalkSpeedCrouched` _charactermovement))
  (if (`Actor.HasAuthority` _returnvalue)
    (bind _returnvalue_2 (`|AddComponentByClass` _returnvalue "/Script/Engine.PhysicsHandleComponent"))
    (bind _asphysics_handle_component (cast `PhysicsHandleComponent` _returnvalue_2))
    (bind _output_get_2 (set `self.Handle` _asphysics_handle_component))
    (`PhysicsHandleComponent.SetLinearStiffness` _output_get_2 750.0)
    (`PhysicsHandleComponent.SetLinearDamping` _output_get_2 200.0)
    (`PhysicsHandleComponent.SetInterpolationSpeed` _output_get_2 30.0)))

(event `self.ReceiveEndPlay`
  (params (EndPlayReason :type "EEndPlayReason Enum" :default "Destroyed"))
  (`self.StopCarry`))

(event `EnhancedInput|/Game/Input/Actions/IA_Drop`
  (params (ActionValue :type Boolean) (ElapsedSeconds :type "Float (double-precision)") (TriggeredSeconds :type "Float (double-precision)") (InputAction :type "InputAction Object Reference" :default "/Game/Input/Actions/IA_Drop.IA_Drop"))
  ; Drop
  (:`Started`
    (`self.Server_Release`)))

(event `Server_Release`
  ; Drop
  (`self.StopCarry`))

(event `EnhancedInput|/Game/Input/Actions/IA_Throw`
  (params (ActionValue :type Boolean) (ElapsedSeconds :type "Float (double-precision)") (TriggeredSeconds :type "Float (double-precision)") (InputAction :type "InputAction Object Reference" :default "/Game/Input/Actions/IA_Throw.IA_Throw"))
  ; Throw
  (:`Started`
    (`self.Server_Throw`)))

(event `Server_Throw`
  (bind _carriedloot (`self.CarriedLoot`))
  ; Throw
  (`/Engine/EditorBlueprintResources/StandardMacros.IsValid` _carriedloot
    (:`Is Valid`
      (set `self.ThrownLoot` _carriedloot)
      (`self.StopCarry`)
      (`PrimitiveComponent.AddImpulse` (`/Game/OurStuff/Blueprints/BP_InteractMaster.Mesh` (`self.ThrownLoot`)) (* (`KismetMathLibrary.Normal` (+ (`KismetMathLibrary.GetForwardVector` (`.OutRotation` (`Actor.GetActorEyesViewPoint` (`self.OwnerPawn`)))) (0.0 0.0 0.25))) (`self.ThrowImpulse`)) "None" false)
      (set `self.ThrownLoot` null))))

(fn `OnRep_SpeedMultiplier`
  (bind _asbp_robber_character (cast `/Game/OurStuff/Core/Player/Game/BP_RobberCharacter` (`self.OwnerPawn`)))
  (set `ProductionGameCharacter.MoveSpeedMultiplier` (`self.SpeedMultiplier`) _asbp_robber_character)
  (set `CharacterMovementComponent.MaxWalkSpeedCrouched` (* (`self.BaseCrouchSpeed`) (`self.SpeedMultiplier`)) (`Character.CharacterMovement` _asbp_robber_character)))

(fn `SetCarrySpeed`
  (params (Multiplier :type "Float (double-precision)"))
  (set `self.SpeedMultiplier` Multiplier))

(fn `StartCarry`
  (params (Loot :type "/Game/OurStuff/Blueprints/Props/Loot/BP_LootBase Object Reference"))
  (locals (GrabPoint :type "Vector Structure"))
  (bind _returnvalue (`self.GetOwner`))
  (bind _carriedloot (`self.CarriedLoot`))
  (bind _mesh (`/Game/OurStuff/Blueprints/BP_InteractMaster.Mesh` Loot))
  (bind _grabpoint (`local.GrabPoint`))
  (bind _mesh_2 (`/Game/OurStuff/Blueprints/BP_InteractMaster.Mesh` Loot))
  (bind _returnvalue_2 (`SceneComponent.K2_GetComponentRotation` _mesh_2))
  (bind (_outlocation _outrotation) (`Actor.GetActorEyesViewPoint` (`self.OwnerPawn`)))
  (if (`Actor.HasAuthority` _returnvalue)
    (if (not (== _carriedloot Loot))
      (`/Engine/EditorBlueprintResources/StandardMacros.IsValid` _carriedloot
        (:`Is Valid`
          (`self.StopCarry`))
        (:`Is Not Valid`
          _))
      (bind (_outhit _returnvalue_3) (`KismetSystemLibrary.LineTraceSingle` _outlocation (+ _outlocation (* (`KismetMathLibrary.GetForwardVector` _outrotation) 200.0)) "TraceTypeQuery1" false (`|MakeArray` _returnvalue) "ForOneFrame"))
      (bind (_bblockinghit _binitialoverlap _time _distance _location _impactpoint _normal _impactnormal _physmat _hitactor) (`GameplayStatics.BreakHitResult` _outhit))
      (set `local.GrabPoint` (`KismetMathLibrary.SelectVector` _impactpoint (`SceneComponent.K2_GetComponentLocation` _mesh) (and _returnvalue_3 (== _hitactor Loot))))
      (if (<= (`/Game/OurStuff/Blueprints/Props/Loot/BP_LootBase.Weight` Loot) (`self.LiftLimit`))
        (`PhysicsHandleComponent.GrabComponentAtLocationWithRotation` (`self.Handle`) _mesh_2 "None" (`local.GrabPoint`) _returnvalue_2)
        (set `self.HoldUpright` true)
        (set `self.HoldRotOffset` (`KismetMathLibrary.NormalizedDeltaRotator` _returnvalue_2 (`KismetMathLibrary.MakeRotator` 0.0 0.0 (.yaw _outrotation))))
        (else
          (`PhysicsHandleComponent.GrabComponentAtLocation` (`self.Handle`) _mesh "None" _grabpoint)
          (set `self.HoldUpright` false)))
      (set `self.GrabOffsetLocal` (`KismetMathLibrary.InverseTransformLocation` (`SceneComponent.K2_GetComponentToWorld` _mesh) _grabpoint))
      (bind _output_get (set `self.CarriedLoot` Loot))
      (`/Game/OurStuff/Blueprints/Props/Loot/BP_LootBase.AddHolder` _output_get (`self.GetOwner`)))))

(fn `StopCarry`
  (`/Engine/EditorBlueprintResources/StandardMacros.IsValid` (`self.CarriedLoot`)
    (:`Is Valid`
      (`PhysicsHandleComponent.ReleaseComponent` (`self.Handle`))
      (`/Game/OurStuff/Blueprints/Props/Loot/BP_LootBase.RemoveHolder` (`self.CarriedLoot`) (`self.GetOwner`))
      (`self.SetCarrySpeed` 1.0)
      (set `self.CarriedLoot` null))))