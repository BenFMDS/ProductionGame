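; Interaction component for a player pawn that detects interactable actors in view and lets the player use them.
; Tick finds the locally controlled owner's WBP_Interaction widget, then traces a short ray from camera 0 each frame.
; BPI_Interaction hits supply the widget's prompt data, and Item or NPC tagged BP_InteractMaster hits get a custom-depth outline.
; IA_Interact, after a brief delay, sends InteractMessage locally and again through a server event.
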(event `self.ReceiveBeginPlay`)

(event `self.ReceiveTick`
  (params (DeltaSeconds :type "Float (single-precision)"))
  (if (`KismetSystemLibrary.IsValid` (`self.Interaction Widget Ref`))
    (`self.LineTrace`)
    (else
      (`self.FindMyWidget`))))

(event `EnhancedInput|/Game/Input/Actions/IA_Interact`
  (params (ActionValue :type Boolean) (ElapsedSeconds :type "Float (double-precision)") (TriggeredSeconds :type "Float (double-precision)") (InputAction :type "InputAction Object Reference" :default "/Game/Input/Actions/IA_Interact.IA_Interact"))
  (:`Started`
    (`KismetSystemLibrary.Delay` 0.1)
    (`self.InteractActor`
      (:`then`
        (message `/Game/OurStuff/Core/InteractionSystem/BPI_Interaction.Interact` (`self.InteractActor`) (`self.GetOwner`) false)
        (`self.Server_Interact` (`self.InteractActor`) (`self.GetOwner`)))
      (:`else`))))

(event `Server_Interact`
  (params (Target :type "Object Object Reference") (InteractingPlayer :type "Actor Object Reference"))
  (message `/Game/OurStuff/Core/InteractionSystem/BPI_Interaction.Interact` Target InteractingPlayer true))

(fn `FindMyWidget`
  (bind _aspawn (cast `Pawn` (`self.GetOwner`)))
  (if (`Pawn.IsLocallyControlled` _aspawn)
    (bind _foundwidgets (`WidgetBlueprintLibrary.GetAllWidgetsOfClass` "/Game/OurStuff/Core/InteractionSystem/WBP_Interaction.WBP_Interaction_C"))
    (for _array_element _foundwidgets
      (bind _returnvalue (`Widget.GetOwningPlayer` _array_element))
      (if (and (== _returnvalue (`Pawn.GetController` _aspawn)) (`KismetSystemLibrary.IsValid` _returnvalue))
        (set `self.Interaction Widget Ref` _array_element)
        (else
          (`KismetSystemLibrary.PrintString` "False"))))))

(fn `LineTrace`
  (bind _returnvalue (`GameplayStatics.GetPlayerCameraManager` 0))
  (bind _interaction_widget_ref (`self.Interaction Widget Ref`))
  (bind _returnvalue_2 (`Actor.K2_GetActorLocation` _returnvalue))
  (bind (_outhit _returnvalue_3) (`KismetSystemLibrary.LineTraceSingle` _returnvalue_2 (+ _returnvalue_2 (* (`Actor.GetActorForwardVector` _returnvalue) 300.0)) "TraceTypeQuery1"))
  (if _returnvalue_3
    (bind (_bblockinghit _binitialoverlap _time _distance _location _impactpoint _normal _impactnormal _physmat _hitactor) (`GameplayStatics.BreakHitResult` _outhit))
    (`RobberInteractable.ClearStaleOutline` (`self.Hit Actor`) _hitactor)
    (set `self.Hit Actor` _hitactor)
    (if (`KismetSystemLibrary.DoesImplementInterface` _hitactor "/Game/OurStuff/Core/InteractionSystem/BPI_Interaction.BPI_Interaction_C")
      (bind _output_get (set `self.InteractActor` _hitactor))
      (bind _interacttext (message `/Game/OurStuff/Core/InteractionSystem/BPI_Interaction.GetInteractData` _output_get))
      (`/Game/OurStuff/Core/InteractionSystem/WBP_Interaction.UpdateWidget` _interaction_widget_ref true _interacttext)
      (if (or (`Actor.ActorHasTag` _hitactor "Item") (`Actor.ActorHasTag` _hitactor "NPC"))
        (bind _asbp_interact_master (cast `/Game/OurStuff/Blueprints/BP_InteractMaster` (`self.Hit Actor`)))
        (`PrimitiveComponent.SetRenderCustomDepth` (`/Game/OurStuff/Blueprints/BP_InteractMaster.Mesh` _asbp_interact_master) true))
      (else
        (`self.InteractActor` :!label _label
          (:`then`
            (set `self.InteractActor` null)
            (`/Game/OurStuff/Core/InteractionSystem/WBP_Interaction.UpdateWidget` _interaction_widget_ref false "")
            (bind _hit_actor (`self.Hit Actor`)
              (:`then`
                (bind _asbp_interact_master_2 (cast `/Game/OurStuff/Blueprints/BP_InteractMaster` _hit_actor))
                (`PrimitiveComponent.SetRenderCustomDepth` (`/Game/OurStuff/Blueprints/BP_InteractMaster.Mesh` _asbp_interact_master_2) false))
              (:`else`)))
          (:`else`))))
    (else
      (goto _label))))