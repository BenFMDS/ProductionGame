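; AI controller for dialogue that runs a dialogue behavior tree and switches it between idle and talking states.
; On BeginPlay it finds the BP_TalkingMaster actor in the level, runs that actor's DialogueTree, then sets itself idle.
; SetStateAsIdle and SetStateAsTalking write the AI state enum to the blackboard, with the talking call also storing the target object for the tree to use.
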(event `self.ReceiveBeginPlay`
  (bind _returnvalue (`GameplayStatics.GetActorOfClass` "/Game/OurStuff/Blueprints/TalkingNPCs/BP_TalkingMaster.BP_TalkingMaster_C"))
  (`self.RunBehaviorTree` (`/Game/OurStuff/Blueprints/TalkingNPCs/BP_TalkingMaster.DialogueTree` _returnvalue))
  (`self.SetStateAsIdle`))

(fn `SetStateAsIdle`
  (`BlackboardComponent.SetValueAsEnum` (`self.Blackboard`) (`self.AIStateKeyName`) (enumliteral `/Game/OurStuff/Core/Dialogue/E_AIState` "NewEnumerator0")))

(fn `SetStateAsTalking`
  (params (Target :type "Actor Object Reference"))
  (`BlackboardComponent.SetValueAsEnum` (`self.Blackboard`) (`self.AIStateKeyName`) (enumliteral `/Game/OurStuff/Core/Dialogue/E_AIState` "NewEnumerator1"))
  (`BlackboardComponent.SetValueAsObject` (`self.Blackboard`) (`self.TargetKeyName`) Target))

(fn `UserConstructionScript`)