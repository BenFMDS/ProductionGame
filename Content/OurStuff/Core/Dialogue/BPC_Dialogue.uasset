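; Actor component that runs dialogue for an AI-controlled owner, caching its dialogue controller and the robber player character on BeginPlay.
; CreateTextDisplay opens a single text display widget using the component's name and texture, shows the cursor in UI-only input, and sets the controller to talking toward the player.
; EndDialogue removes the widget, restores game-only input, and returns the controller to idle.
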(event `self.ReceiveBeginPlay`
  (bind _asbp_dailogue_controller (cast `/Game/OurStuff/Core/Dialogue/AI/BP_DailogueController` (`AIBlueprintHelperLibrary.GetAIController` (`self.GetOwner`))))
  (set `self.DailogueControllerRef` _asbp_dailogue_controller)
  (bind _returnvalue (`GameplayStatics.GetActorOfClass` "/Game/OurStuff/Core/Player/Game/BP_RobberCharacter.BP_RobberCharacter_C"))
  (set `self.PlayerRef` _returnvalue))

(event `CreateTextDisplay`
  (bind _returnvalue (`GameplayStatics.GetPlayerController` 0))
  (`/Engine/EditorBlueprintResources/StandardMacros.IsValid` (`self.TextDisplayRef`)
    (:`Is Not Valid`
      (bind _returnvalue_2 (`|CreateWidget` "/Game/OurStuff/Core/Dialogue/WBP_TextDisplay.WBP_TextDisplay_C" null (`self.Name`) (`self.Texture`)))
      (`KismetSystemLibrary.PrintString` "Created Widget")
      (bind _output_get (set `self.TextDisplayRef` _returnvalue_2))
      (`UserWidget.AddToViewport` _output_get 0)
      (`WidgetBlueprintLibrary.SetInputMode_UIOnlyEx` _returnvalue _output_get)
      (set `PlayerController.bShowMouseCursor` true _returnvalue)
      (bind _dailoguecontrollerref (`self.DailogueControllerRef`)
        (:`then`
          (`/Game/OurStuff/Core/Dialogue/AI/BP_DailogueController.SetStateAsTalking` _dailoguecontrollerref (`self.PlayerRef`)))
        (:`else`)))))

(event `EndDialogue`
  (bind _returnvalue (`GameplayStatics.GetPlayerController` 0))
  (bind _textdisplayref (`self.TextDisplayRef`))
  (`/Engine/EditorBlueprintResources/StandardMacros.IsValid` _textdisplayref
    (:`Is Valid`
      (`Widget.RemoveFromParent` _textdisplayref)
      (`WidgetBlueprintLibrary.SetInputMode_GameOnly` _returnvalue)
      (set `PlayerController.bShowMouseCursor` false _returnvalue)
      (set `self.TextDisplayRef` null)
      (bind _dailoguecontrollerref (`self.DailogueControllerRef`)
        (:`then`
          (`/Game/OurStuff/Core/Dialogue/AI/BP_DailogueController.SetStateAsIdle` _dailoguecontrollerref))
        (:`else`)))))