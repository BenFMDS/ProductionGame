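; AI controller for BP_Guard that runs BT_Guard and drives sight-based detection of player-controlled robbers.
; Each tick it raises the detection meter while a robber is seen, slower if player 0 crouches, and drains it otherwise.
; Detection and lost-sight time drive guard states, synced to the Blackboard, setting speed, focus and rotation.
; Robbers within catch radius during Chase teleport to a PlayerStart, resetting the guard to Patrol.
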(event `self.ReceivePossess`
  (params (PossessedPawn :type "Pawn Object Reference"))
  (bind _asbp_guard (cast `/Game/OurStuff/Guard/BP_Guard` PossessedPawn))
  (set `self.Guard` _asbp_guard)
  (`self.RunBehaviorTree` "/Game/OurStuff/Guard/Behaviour/BT_Guard.BT_Guard")
  (`KismetSystemLibrary.PrintString` "Guard Possessed"))

(event `self.ReceiveTick`
  (params (DeltaSeconds :type "Float (single-precision)"))
  (`self.UpdateDetection` DeltaSeconds))

(fn `CatchRobber`
  (params (Robber :type "Actor Object Reference"))
  (`KismetSystemLibrary.PrintString` (`KismetStringLibrary.Concat_StrStr` "Caught " (`KismetSystemLibrary.GetDisplayName` Robber)))
  (bind _returnvalue (`GameplayStatics.GetActorOfClass` "/Script/Engine.PlayerStart"))
  (`self.K2_TeleportTo` Robber (`self.K2_GetActorLocation` _returnvalue) (`self.K2_GetActorRotation` _returnvalue))
  (`BlackboardComponent.ClearValue` (`AIBlueprintHelperLibrary.GetBlackboard` null) "TargetActor")
  (set `/Game/OurStuff/Guard/BP_Guard.Detection` 0.0 (`self.Guard`))
  (set `self.TimeSinceSeen` 0.0)
  (`self.SetGuardState` "NewEnumerator0"))

(fn `FindSeenRobber`
  (returns (Robber :type "Character Object Reference"))
  (locals (Best :type "Character Object Reference") (BestDistance :type "Float (double-precision)" :default 9999999.0))
  (set `self.SeenActors` (`AIPerceptionComponent.GetCurrentlyPerceivedActors` (`self.AIPerception`) "/Script/AIModule.AISense_Sight"))
  (bind _ascharacter (cast `Character` (`BlackboardComponent.GetValueAsObject` (`AIBlueprintHelperLibrary.GetBlackboard` null) "TargetActor"))
    (:`then`
      (if (`KismetArrayLibrary.Array_Contains` (`self.SeenActors`) _ascharacter)
        (return _ascharacter)
        (else
          _)))
    (:`CastFailed`
      _))
  (for _array_element (`self.SeenActors`)
    (bind _ascharacter_2 (cast `Character` _array_element))
    (if (`Pawn.IsPlayerControlled` _ascharacter_2)
      (bind _returnvalue (`self.GetDistanceTo` _ascharacter_2 (`self.Guard`)))
      (if (< _returnvalue (`local.BestDistance`))
        (bind _output_get (set `local.Best` _ascharacter_2))
        (set `local.BestDistance` _returnvalue)
        (return _output_get)))))

(fn `SetGuardState`
  (params (NewState :type "/Game/OurStuff/Guard/E_GuardState Enum" :default "NewEnumerator0"))
  (locals (KeyName :type Name :default "GuardState"))
  (bind _guard (`self.Guard`))
  (bind _guard_2 (`self.Guard`))
  (bind _guard_3 (`self.Guard`))
  (bind _guard_4 (`self.Guard`))
  (if (`|EnumInequality` NewState (`/Game/OurStuff/Guard/BP_Guard.GuardState` _guard_4))
    (`BlackboardComponent.SetValueAsEnum` (`AIBlueprintHelperLibrary.GetBlackboard` null) (`local.KeyName`) NewState)
    (bind _output_get (set `/Game/OurStuff/Guard/BP_Guard.GuardState` NewState _guard_4))
    (switch `/Game/OurStuff/Guard/E_GuardState` _output_get
      (:`NewEnumerator0`
        (set `CharacterMovementComponent.MaxWalkSpeed` (`/Game/OurStuff/Guard/BP_Guard.WalkSpeed` _guard) (`Character.CharacterMovement` _guard))
        (`self.K2_ClearFocus`)
        (`self.SetRotationMode` false))
      (:`NewEnumerator1`
        (`self.StopMovement`)
        (bind _asactor (cast `Actor` (`BlackboardComponent.GetValueAsObject` (`AIBlueprintHelperLibrary.GetBlackboard` null) "TargetActor")))
        (`self.K2_SetFocus` _asactor)
        (`self.SetRotationMode` true))
      (:`NewEnumerator2`
        (set `CharacterMovementComponent.MaxWalkSpeed` (`/Game/OurStuff/Guard/BP_Guard.InvestigateSpeed` _guard_2) (`Character.CharacterMovement` _guard_2))
        (`self.K2_ClearFocus`)
        (`self.SetRotationMode` false))
      (:`NewEnumerator3`
        (set `CharacterMovementComponent.MaxWalkSpeed` (`/Game/OurStuff/Guard/BP_Guard.RunSpeed` _guard_3) (`Character.CharacterMovement` _guard_3))
        (`self.K2_ClearFocus`)
        (`self.SetRotationMode` false)))))

(fn `SetRotationMode`
  (params (FaceTarget :type Boolean))
  (bind _charactermovement (`Character.CharacterMovement` (`self.Guard`)))
  (set `CharacterMovementComponent.bOrientRotationToMovement` (not FaceTarget) _charactermovement)
  (set `CharacterMovementComponent.bUseControllerDesiredRotation` FaceTarget _charactermovement))

(fn `UpdateDetection`
  (params (DeltaSeconds :type "Float (double-precision)"))
  (locals (Seen :type "Character Object Reference") (Rate :type "Float (double-precision)") (Target :type "Actor Object Reference"))
  (bind _guard (`self.Guard`))
  (bind _guard_2 (`self.Guard`))
  (bind _guard_3 (`self.Guard`))
  (bind _guard_4 (`self.Guard`))
  (bind _guard_5 (`self.Guard`))
  (bind _guardstate (`/Game/OurStuff/Guard/BP_Guard.GuardState` (`self.Guard`)))
  (bind _guardstate_2 (`/Game/OurStuff/Guard/BP_Guard.GuardState` _guard_2))
  (`/Engine/EditorBlueprintResources/StandardMacros.IsValid` (`self.Guard`)
    (:`Is Valid`
      (bind _asactor (cast `Actor` (`BlackboardComponent.GetValueAsObject` (`AIBlueprintHelperLibrary.GetBlackboard` null) "TargetActor"))
        (:`then`
          (set `local.Target` _asactor))
        (:`CastFailed`
          _))
      (if (and (`|EnumEquality` (`/Game/OurStuff/Guard/BP_Guard.GuardState` _guard_4) "NewEnumerator3") (`KismetSystemLibrary.IsValid` (`local.Target`)) (<= (`self.GetDistanceTo` _guard_4 (`local.Target`)) (`self.CatchRadius`)))
        (`self.CatchRobber` (`local.Target`))
        (return)
        (else
          (bind _robber (`self.FindSeenRobber`))
          (bind _output_get (set `local.Seen` _robber))
          (if (`KismetSystemLibrary.IsValid` _output_get)
            ; True Branch: Someone is Seen
            (`BlackboardComponent.SetValueAsObject` (`AIBlueprintHelperLibrary.GetBlackboard` null) "TargetActor" (`local.Seen`))
            (`BlackboardComponent.SetValueAsVector` (`AIBlueprintHelperLibrary.GetBlackboard` null) "LastKnownLocation" (`self.K2_GetActorLocation` (`local.Seen`)))
            (set `self.TimeSinceSeen` 0.0)
            ;; Fill Rate: Crouch Multiplier Reduces the Detection Rate
            (set `local.Rate` (* (`self.DetectionRateUp`) (`KismetMathLibrary.SelectFloat` (`self.CrouchMultiplier`) 1.0 (`Character.bIsCrouched` (`GameplayStatics.GetPlayerCharacter` 0)))))
            (set `/Game/OurStuff/Guard/BP_Guard.Detection` (`KismetMathLibrary.FClamp` (+ (`/Game/OurStuff/Guard/BP_Guard.Detection` _guard_5) (* (`local.Rate`) DeltaSeconds)) 0.0 (`/Game/OurStuff/Guard/BP_Guard.DetectionMax` _guard_5)) (`self.Guard`))
            ;; Set Guard States
            (if (>= (`/Game/OurStuff/Guard/BP_Guard.Detection` _guard_3) (`/Game/OurStuff/Guard/BP_Guard.DetectionMax` _guard_3))
              (`self.SetGuardState` "NewEnumerator3")
              (elif (or (`|EnumEquality` _guardstate "NewEnumerator0") (`|EnumEquality` _guardstate "NewEnumerator2"))
                (`self.SetGuardState` "NewEnumerator1")))
            (else
              ; False Branch: Nobody is Seen
              (set `self.TimeSinceSeen` (+ (`self.TimeSinceSeen`) DeltaSeconds))
              (set `/Game/OurStuff/Guard/BP_Guard.Detection` (`KismetMathLibrary.FClamp` (- (`/Game/OurStuff/Guard/BP_Guard.Detection` _guard) (* (`self.DetectionRateDown`) DeltaSeconds)) 0.0 (`/Game/OurStuff/Guard/BP_Guard.DetectionMax` _guard)) _guard_2)
              (if (and (or (`|EnumEquality` _guardstate_2 "NewEnumerator1") (`|EnumEquality` _guardstate_2 "NewEnumerator3")) (>= (`self.TimeSinceSeen`) (`self.LoseSightTime`)))
                (`self.SetGuardState` "NewEnumerator0")))))))
    (:`Is Not Valid`
      (return))))

(fn `UserConstructionScript`)