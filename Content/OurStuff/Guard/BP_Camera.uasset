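; Security camera for stealth gameplay that detects the player and reports a catch to the game mode.
; Each tick, a view-cone and line-trace check, combined with player visibility, fills or drains a detection meter shown on a camera-facing widget bar.
; The meter drives a three-state alert that plays a suspicion sound and calls OnPlayerCaught when full.
; Patrol only resets its index, and turning toward the player is never run.
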(event `self.ReceiveTick`
  (params (DeltaSeconds :type "Float (single-precision)"))
  (`self.UpdateDetection` DeltaSeconds)
  (`self.RotateDetectionBar`)
  (bind _returnvalue (`self.CanSeePlayer`))
  (set `self.bPlayerDetected` _returnvalue)
  (if (== (`self.GuardState`) 1)
    _))

(event `self.ReceiveBeginPlay`
  (bind _aswbp_camera_detection (cast `/Game/OurStuff/Guard/WBP_CameraDetection` (`WidgetComponent.GetUserWidgetObject` (`self.DetectionBar`))))
  (set `/Game/OurStuff/Guard/WBP_CameraDetection.CameraRef` self _aswbp_camera_detection)
  (bind _asbp_first_person_character (cast `/Game/FirstPerson/Blueprints/BP_FirstPersonCharacter` (`GameplayStatics.GetPlayerCharacter` 0)))
  (set `self.As BP First Person Character` _asbp_first_person_character)
  (`self.Start Patrol`))

(event `Start Patrol`
  (set `self.CurrentPatrolIndex` 0))

(fn `CanSeePlayer`
  (returns (ReturnValue :type Boolean))
  (bind _returnvalue (`self.K2_GetActorLocation`))
  (bind _returnvalue_2 (+ (`self.K2_GetActorLocation`) (0.0 0.0 60.0)))
  (bind _asbp_first_person_character (cast `/Game/FirstPerson/Blueprints/BP_FirstPersonCharacter` (`GameplayStatics.GetPlayerCharacter` 0)))
  (bind _output_get (set `self.As BP First Person Character` _asbp_first_person_character))
  (`/Engine/EditorBlueprintResources/StandardMacros.IsValid` _output_get
    (:`Is Valid`
      (bind _returnvalue_3 (`self.K2_GetActorLocation` _output_get))
      (bind _returnvalue_4 (`KismetMathLibrary.Normal` (- _returnvalue _returnvalue_3)))
      (if (>= (`KismetMathLibrary.Dot_VectorVector` (* (`self.GetActorForwardVector`) -1.0) _returnvalue_4) (`KismetMathLibrary.Cos` (`KismetMathLibrary.DegreesToRadians` (`self.VisionAngle`))))
        (bind (_outhit _returnvalue_5) (`KismetSystemLibrary.LineTraceSingle` :`Start` _returnvalue_2 :`End` (+ _returnvalue_2 (* (* _returnvalue_4 -1.0) (`self.VisionDistance`))) :`TraceChannel` "TraceTypeQuery1" :`DrawTime` 1.0))
        (if _returnvalue_5
          (return (== (`.HitActor` (`GameplayStatics.BreakHitResult` _outhit)) (`self.As BP First Person Character`))))))
    (:`Is Not Valid`
      (return (<= (`KismetMathLibrary.Vector_Distance` _returnvalue _returnvalue_3) (`self.VisionDistance`))))))

(fn `RotateDetectionBar`
  (bind _detectionbar (`self.DetectionBar`))
  (`SceneComponent.K2_SetWorldRotation` _detectionbar (`KismetMathLibrary.FindLookAtRotation` (`SceneComponent.K2_GetComponentLocation` _detectionbar) (`PlayerCameraManager.GetCameraLocation` (`PlayerController.PlayerCameraManager` (`GameplayStatics.GetPlayerController` 0)))) false false))

(fn `RotateTowardPlayer`
  (`/Engine/EditorBlueprintResources/StandardMacros.IsValid` (`self.As BP First Person Character`)
    (:`Is Valid`
      (`self.K2_SetActorRotation` (`KismetMathLibrary.RInterpTo` (`self.K2_GetActorRotation`) (`KismetMathLibrary.MakeRotator` 0.0 0.0 (.yaw (`KismetMathLibrary.FindLookAtRotation` (`self.K2_GetActorLocation`) (`self.K2_GetActorLocation` (`self.As BP First Person Character`))))) (`GameplayStatics.GetWorldDeltaSeconds`) (`self.TurnSpeed`))))))

(fn `UpdateDetection`
  (params (InputPin :type "Float (single-precision)"))
  (bind _as_bp_first_person_character (`self.As BP First Person Character`))
  (bind _detectionbar (`self.DetectionBar`))
  (if (`|EnumInequality` (`self.GuardState`) "NewEnumerator2")
    (`/Engine/EditorBlueprintResources/StandardMacros.IsValid` _as_bp_first_person_character
      (:`Is Valid`
        (bind _returnvalue (`self.CanSeePlayer`))
        (if (and (`/Game/FirstPerson/Blueprints/BP_FirstPersonCharacter.PlayerVisable` _as_bp_first_person_character) _returnvalue)
          (set `self.Detection` (`KismetMathLibrary.FClamp` (+ (`self.Detection`) (* (`self.DetectionRateUp`) InputPin)) 0.0 (`self.DetectionMax`)))
          (else
            (set `self.Detection` (`KismetMathLibrary.FClamp` (- (`self.Detection`) (* (`self.DetectionRateDown`) (`GameplayStatics.GetWorldDeltaSeconds`))) 0.0 (`self.DetectionMax`)))))
        (if (> (`self.Detection`) 0.0)
          (`SceneComponent.SetVisibility` _detectionbar true false)
          (else
            (`SceneComponent.SetVisibility` _detectionbar false false)))
        (if (and (== (`self.GuardState`) 0) (> (`self.Detection`) 20.0))
          (set `self.GuardState` "NewEnumerator1")
          (`GameplayStatics.PlaySoundAtLocation` (`self.SuspicousSound`) (`self.K2_GetActorLocation`) (struct) 1.0 1.0 0.0 null null null null)
          (elif (and (== (`self.GuardState`) 1) (== (`self.Detection`) 0.0))
            (set `self.GuardState` "NewEnumerator0")
            (elif (>= (`self.Detection`) (`self.DetectionMax`))
              (set `self.GuardState` "NewEnumerator2")
              (bind _asbp_first_person_game_mode (cast `/Game/FirstPerson/Blueprints/BP_FirstPersonGameMode` (`GameplayStatics.GetGameMode`)))
              (`/Game/FirstPerson/Blueprints/BP_FirstPersonGameMode.OnPlayerCaught` _asbp_first_person_game_mode))))))))

(fn `UserConstructionScript`)