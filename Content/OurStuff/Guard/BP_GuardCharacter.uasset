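; Guard character that patrols points and detects the player robber in a stealth game.
; AIMoveTo loops through patrol points, pausing to look around at each.
; Each tick, a view-cone and line-trace check, plus robber visibility, raises or drains a detection meter shown on a camera-facing widget.
; The meter drives a three-state enum: patrolling, suspicious (stops, plays sound, turns toward player) until fully drained, and a final state at maximum that freezes detection updates.
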(event `self.ReceiveTick`
  (params (DeltaSeconds :type "Float (single-precision)"))
  (`self.UpdateDetection` DeltaSeconds)
  (`self.RotateDetectionBar`)
  (bind _returnvalue (`self.CanSeePlayer`))
  (set `self.bPlayerDetected` _returnvalue)
  (if (== (`self.GuardState`) 1)
    (`self.RotateTowardPlayer`)))

(event `self.ReceiveBeginPlay`
  (bind _aswbp_guard_detection (cast `/Game/OurStuff/Guard/WBP_GuardDetection` (`WidgetComponent.GetUserWidgetObject` (`self.DetectionBar`))))
  (set `/Game/OurStuff/Guard/WBP_GuardDetection.GuardRef` self _aswbp_guard_detection)
  (bind _asbp_robber_character (cast `/Game/OurStuff/Core/Player/Game/BP_RobberCharacter` (`GameplayStatics.GetPlayerCharacter` 0)))
  (set `self.BP_RobberCharacter` _asbp_robber_character)
  (`self.Start Patrol`))

(event `AdvanceIndex`
  (bind _result (`/Engine/EditorBlueprintResources/StandardMacros.IncrementInt` (`self.CurrentPatrolIndex`))
    (:`  `
      (if (>= _result (`KismetArrayLibrary.Array_Length` (`self.PatrolPoints`)))
        (set `self.CurrentPatrolIndex` 0)))))

(event `Start Patrol`
  (set `self.CurrentPatrolIndex` 0)
  (`self.MoveToCurrentPoint`))

(event `MoveToCurrentPoint`
  (`SkeletalMeshComponent.PlayAnimation` (`self.Mesh`) "/Game/OurStuff/Guard/Animations/Walking_BOXMAN_Anim.Walking_BOXMAN_Anim" true)
  (if (> (`KismetArrayLibrary.Array_Length` (`self.PatrolPoints`)) 0)
    (if (== (`self.GuardState`) 0)
      (`|AIMoveTo` self (`self.K2_GetActorLocation` (`|GetArrayItem` (`self.PatrolPoints`) (`self.CurrentPatrolIndex`))) null
        (:`OnSuccess`
          (`self.OnReachPoint`))
        (:`OnFail`
          (`self.AdvanceIndex`)
          (`self.MoveToCurrentPoint`))))))

(event `OnReachPoint`
  (`SkeletalMeshComponent.PlayAnimation` (`self.Mesh`) "/Game/OurStuff/Guard/Animations/Looking_right_to_left_BOXMAN_Anim.Looking_right_to_left_BOXMAN_Anim" false)
  (set `self.bIsWaiting` true)
  (`KismetSystemLibrary.Delay` (`self.WaitTime`))
  (set `self.bIsWaiting` false)
  (`self.AdvanceIndex`)
  (`self.MoveToCurrentPoint`))

(fn `CanSeePlayer`
  (returns (ReturnValue :type Boolean))
  (bind _returnvalue (`self.K2_GetActorLocation`))
  (bind _returnvalue_2 (`self.K2_GetActorLocation`))
  (bind _returnvalue_3 (+ (`self.K2_GetActorLocation`) (0.0 0.0 60.0)))
  (bind _returnvalue_4 (`KismetMathLibrary.Normal` (- _returnvalue_2 _returnvalue)))
  (bind _asbp_robber_character (cast `/Game/OurStuff/Core/Player/Game/BP_RobberCharacter` (`GameplayStatics.GetPlayerCharacter` 0)))
  (bind _output_get (set `self.BP_RobberCharacter` _asbp_robber_character))
  (`/Engine/EditorBlueprintResources/StandardMacros.IsValid` _output_get
    (:`Is Valid`
      (if (>= (`KismetMathLibrary.Dot_VectorVector` (* (`self.GetActorForwardVector`) -1.0) _returnvalue_4) (`KismetMathLibrary.Cos` (`KismetMathLibrary.DegreesToRadians` (`self.VisionAngle`))))
        (bind (_outhit _returnvalue_5) (`KismetSystemLibrary.LineTraceSingle` _returnvalue_3 (+ _returnvalue_3 (* (* _returnvalue_4 -1.0) (`self.VisionDistance`))) "TraceTypeQuery1"))
        (if _returnvalue_5
          (return (== (`.HitActor` (`GameplayStatics.BreakHitResult` _outhit)) (`self.BP_RobberCharacter`))))))
    (:`Is Not Valid`
      (return (<= (`KismetMathLibrary.Vector_Distance` _returnvalue_2 _returnvalue) (`self.VisionDistance`))))))

(fn `RotateDetectionBar`
  (`SceneComponent.K2_SetWorldRotation` (`self.DetectionBar`) (`KismetMathLibrary.FindLookAtRotation` (`SceneComponent.K2_GetComponentLocation` (`self.DetectionBar`)) (`PlayerCameraManager.GetCameraLocation` (`PlayerController.PlayerCameraManager` (`GameplayStatics.GetPlayerController` 0)))) false false))

(fn `RotateTowardPlayer`
  (bind _bp_robbercharacter (`self.BP_RobberCharacter`))
  (`/Engine/EditorBlueprintResources/StandardMacros.IsValid` _bp_robbercharacter
    (:`Is Valid`
      (`self.K2_SetActorRotation` (`KismetMathLibrary.RInterpTo` (`self.K2_GetActorRotation`) (`KismetMathLibrary.MakeRotator` 0.0 0.0 (.yaw (`KismetMathLibrary.FindLookAtRotation` (`self.K2_GetActorLocation`) (`self.K2_GetActorLocation` _bp_robbercharacter)))) (`GameplayStatics.GetWorldDeltaSeconds`) (`self.TurnSpeed`))))))

(fn `UpdateDetection`
  (params (InputPin :type "Float (single-precision)"))
  (bind _returnvalue (`self.GetController`))
  (bind _detectionbar (`self.DetectionBar`))
  (bind _bp_robbercharacter (`self.BP_RobberCharacter`))
  (if (`|EnumInequality` (`self.GuardState`) "NewEnumerator2")
    (`/Engine/EditorBlueprintResources/StandardMacros.IsValid` _bp_robbercharacter
      (:`Is Valid`
        (bind _returnvalue_2 (`self.CanSeePlayer`))
        (if (and (`/Game/OurStuff/Core/Player/Game/BP_RobberCharacter.PlayerVisable` _bp_robbercharacter) _returnvalue_2)
          (set `self.Detection` (`KismetMathLibrary.FClamp` (+ (`self.Detection`) (* (`self.DetectionRateUp`) InputPin)) 0.0 (`self.DetectionMax`)))
          (else
            (set `self.Detection` (`KismetMathLibrary.FClamp` (- (`self.Detection`) (* (`self.DetectionRateDown`) (`GameplayStatics.GetWorldDeltaSeconds`))) 0.0 (`self.DetectionMax`)))))
        (if (> (`self.Detection`) 0.0)
          (`SceneComponent.SetVisibility` _detectionbar true false)
          (else
            (`SceneComponent.SetVisibility` _detectionbar false false)))
        (if (and (== (`self.GuardState`) 0) (> (`self.Detection`) 20.0))
          (set `self.GuardState` "NewEnumerator1")
          (`Controller.StopMovement` _returnvalue)
          (`GameplayStatics.PlaySoundAtLocation` (`self.SuspicousSound`) (`self.K2_GetActorLocation` _returnvalue) (struct) 1.0 1.0 0.0 null null null null)
          (`SkeletalMeshComponent.PlayAnimation` (`self.Mesh`) "/Game/OurStuff/Guard/Animations/Looking_right_to_left_BOXMAN_Anim.Looking_right_to_left_BOXMAN_Anim" false)
          (elif (and (== (`self.GuardState`) 1) (== (`self.Detection`) 0.0))
            (set `self.GuardState` "NewEnumerator0")
            (`self.MoveToCurrentPoint`)
            (if (!= (`self.GuardState`) 0)
              (return))
            (elif (>= (`self.Detection`) (`self.DetectionMax`))
              (set `self.GuardState` "NewEnumerator2"))))))))

(fn `UserConstructionScript`)